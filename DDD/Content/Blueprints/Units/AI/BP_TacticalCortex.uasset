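; BP_TacticalCortex is the tactical navigation grid for units, storing standable tile nodes in a map of XY columns keyed by height.
; Nodes take edge and standing heights from DT_TileShapeInfo, track occupancy, and answer Euclidean, Manhattan and Chebyshev proximity queries.
; FindMoves scans four cardinal directions within jump range, rejects jumps blocked along a traced spline, and classifies moves by travel distance and edge-height difference, flagging hazardous hard landings.
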(fn `AddNewNode`
  (params (Position :type "IntVector Structure") (TileShape :type "/Game/Data/Procedural/E_TileShapes Enum" :default "NewEnumerator29") (TerrainType :type "/Game/Data/Procedural/E_TerrainTypes Enum" :default "NewEnumerator0"))
  (bind _returnvalue (`|GetDataTableRow` "/Game/Data/Procedural/DT_TileShapeInfo.DT_TileShapeInfo" (`KismetStringLibrary.Conv_StringToName` (`KismetStringLibrary.Conv_ByteToString` TileShape)))
    (:`then`
      (if (`.isStandable_22_456497ED2A94426993A4C13968E66FF4` (break `/Game/Data/Procedural/F_TileShapeInfo` _returnvalue))
        (`self.AddNode` (make `/Game/Data/AI/F_TacticalNode` :`TerrainType` TerrainType :`Unit` null :`UnitHeight` (`.CharacterHeight_7_BE088372A2EA429190A7AF61BF144925` (break `/Game/Data/Procedural/F_TileShapeInfo` _returnvalue)) :`NorthEdgeHeight` (`.EdgeHeightNorth_12_BE954A72A6094E1CB9FAF5F6E8DDC281` (break `/Game/Data/Procedural/F_TileShapeInfo` _returnvalue)) :`EastEdgeHeight` (`.EdgeHeightEast_13_876709F35E9F411A80836974B81E6A3C` (break `/Game/Data/Procedural/F_TileShapeInfo` _returnvalue)) :`SouthEdgeHeight` (`.EdgeHeightSouth_14_BD415720F9934163B0364A05595E7302` (break `/Game/Data/Procedural/F_TileShapeInfo` _returnvalue)) :`WestEdgeHeight` (`.EdgeHeightWest_15_A16278DC7A7546E3A1079846B8888B10` (break `/Game/Data/Procedural/F_TileShapeInfo` _returnvalue))) Position)))
    (:`RowNotFound`
      (`KismetSystemLibrary.PrintString` "tile shape info not found")))
  (return))

(fn `AddNode`
  (params (NewNode :type "/Game/Data/AI/F_TacticalNode Structure") (Location :type "IntVector Structure"))
  (bind (_position _terraintype _occupied _unit _pickups _unitheight _northedgeheight _eastedgeheight _southedgeheight _westedgeheight) (break `/Game/Data/AI/F_TacticalNode` NewNode))
  (bind (_x _y _z) (break `IntVector` Location))
  (bind _navigablepoints (`self.NavigablePoints`))
  (bind _f_tacticalnode (make `/Game/Data/AI/F_TacticalNode` (`/Game/Blueprints/Libraries/BPFL_GlobalData.ToWorldPosition` Location) _terraintype _occupied _unit _pickups _unitheight _northedgeheight _eastedgeheight _southedgeheight _westedgeheight))
  (bind _f_intvector2d (make `/Game/Blueprints/Libraries/F_IntVector2d` _x _y))
  (bind (_value _returnvalue) (`BlueprintMapLibrary.Map_Find` _navigablepoints _f_intvector2d))
  (if _returnvalue
    (`BlueprintMapLibrary.Map_Add` (`.Nodes_9_ADB601575A484309BE75B222EA95378A` (break `/Game/Data/AI/F_TacticalArray` _value)) _z _f_tacticalnode)
    (else
      (`BlueprintMapLibrary.Map_Add` _navigablepoints _f_intvector2d (make `/Game/Data/AI/F_TacticalArray` (`|MakeMap` _z _f_tacticalnode))))))

(fn `ClearOccupiedAt`
  (params (Location :type "IntVector Structure"))
  (returns (Success :type Boolean))
  (bind (_foundnode _isfound) (`self.GetNode` Location))
  (if _isfound
    (bind (_position _terraintype _occupied _unit _pickups _unitheight _northedgeheight _eastedgeheight _southedgeheight _westedgeheight) (break `/Game/Data/AI/F_TacticalNode` _foundnode))
    (`self.AddNode` (make `/Game/Data/AI/F_TacticalNode` _position _terraintype false _unit _pickups _unitheight _northedgeheight _eastedgeheight _southedgeheight _westedgeheight) Location)
    (return true)
    (else
      (return false))))

(fn `FindMoves`
  (params (`Starting Position` :type "Vector Structure") (JumpScore :type Integer))
  (returns (ValidMoves :type "Array of /Game/Data/AI/F_MoveData Structure"))
  (locals (`Possible Moves` :type "Array of /Game/Data/AI/F_MoveData Structure") (StartNode :type "/Game/Data/AI/F_TacticalNode Structure") (StartLocation :type "IntVector Structure") (DestinationLocation :type "IntVector Structure") (HazardAccumulator :type Integer) (MoveCost :type Integer) (CurrentMoveType :type "/Game/Data/AI/E_MoveTypes Enum") (isHardLanding :type Boolean) (CurrentDirection :type "/Game/Data/Procedural/E_Direction Enum") (DesinationNode :type "/Game/Data/AI/F_TacticalNode Structure") (HorizontalTravel :type Integer :default 0) (VerticalTravel :type "Float (double-precision)") (FallDistance :type "Float (double-precision)") (Jump_Score :type Integer) (DestinationWorldLocation :type "Vector Structure"))
  (bind _jumpspline (`self.JumpSpline`))
  (bind (_startedgeheight _destinationnearedgeheightheight _destinationfaredgeheight) (`self.GetEdgeHeightsByDirection` (`local.CurrentDirection`) (`local.StartNode`) (`local.DesinationNode`)))
  ;[0.15 0.15 0.15 0.5 35] Initialize start variables
  (set `local.StartLocation` (`/Game/Blueprints/Libraries/BPFL_GlobalData.ToTilePosition` `Starting Position`))
  (bind _output_get (set `local.Jump_Score` JumpScore))
  (set `local.FallDistance` (* _output_get 0.5 1.25))
  (`KismetArrayLibrary.Array_Clear` (`local.Possible Moves`))
  (bind (_foundnode _isfound) (`self.GetNode` (`local.StartLocation`)))
  (if _isfound
    (set `local.StartNode` _foundnode)
    ;[0.15 0.15 0.15 0.5 35] Main Loop
    (bind _arrayelement (`/Game/Blueprints/Libraries/BPML_Utilities.ForEachLoop_Real` (`|MakeArray` "NewEnumerator0" "NewEnumerator1" "NewEnumerator2" "NewEnumerator3" :!type "/Game/Data/Procedural/E_Direction Enum") :!label _label)
      (:`LoopBody`
        (set `local.CurrentDirection` _arrayelement)
        (bind _index (`/Game/Blueprints/Libraries/BPML_Utilities.ForLoop_Real` 1 (+ (/ (`local.JumpScore`) 2) 1) :!label _label_2)
          (:`LoopBody`
            (set `local.MoveCost` _index)
            (bind _tacticalnodes (`self.FindNodes` (`/Game/Blueprints/Libraries/BPML_VectorMath.Add (IntVector2d)` (`/Game/Blueprints/Libraries/BPML_VectorMath.ToIntVector2d` (`local.StartLocation`)) (`/Game/Blueprints/Libraries/BPML_VectorMath.Scale (IntVector2d)` (`/Game/Blueprints/Libraries/BPML_Math.toUnitVector2d` (`local.CurrentDirection`)) (`KismetMathLibrary.Conv_IntToDouble` _index)))))
            (bind _keys (`BlueprintMapLibrary.Map_Keys` _tacticalnodes))
            (bind _arrayelement_2 (`/Game/Blueprints/Libraries/BPML_Utilities.ForEachLoop_Real` _keys :!label _label_3)
              (:`LoopBody`
                (bind (_foundnode_2 _isfound_2) (`self.GetNode` _arrayelement_2))
                (if _isfound_2
                  ;[0.15 0.15 0.15 0.5 35] Loop body
                  ;; Set remaining current move variables
                  (set `local.DesinationNode` _foundnode_2)
                  (set `local.DestinationLocation` _arrayelement_2)
                  (set `local.DestinationWorldLocation` (+ (`/Game/Blueprints/Libraries/BPFL_GlobalData.ToWorldPosition` _arrayelement_2) (`KismetMathLibrary.MakeVector` 0.0 0.0 (`KismetMathLibrary.Conv_IntToDouble` (`.UnitHeight_20_E95CDC97603540709376EEFBAD8A3F15` (break `/Game/Data/AI/F_TacticalNode` _foundnode_2))))))
                  (set `local.HazardAccumulator` 0)
                  (set `local.HorizontalTravel` (- (`/Game/Blueprints/Libraries/BPML_VectorMath.ManhattenDistance (2d)` (`/Game/Blueprints/Libraries/BPML_VectorMath.ToIntVector2d` (`local.StartLocation`)) (`/Game/Blueprints/Libraries/BPML_VectorMath.ToIntVector2d` (`local.DestinationLocation`))) 1))
                  (set `local.isHardLanding` false)
                  (set `local.VerticalTravel` (`self.GetEdgeHeightGain` (`local.CurrentDirection`) (`local.StartNode`) (`local.DesinationNode`)))
                  ;; Determine if walking
                  (if (`KismetMathLibrary.BooleanNAND` (== (`local.HorizontalTravel`) 0) (`KismetMathLibrary.NearlyEqual_FloatFloat` (`local.VerticalTravel`) 0.0 0.01))
                    ;; Determine if jump is within reach
                    (if (>= (/ (`local.Jump_Score`) 2) (+ (`local.HorizontalTravel`) (`local.VerticalTravel`)))
                      ;;[1.597 -1.388 -0.946 0.5] Determine if jump is blocked
                      (bind (_jumpspline_2 _success) (`/Game/Blueprints/Libraries/BPFL_Splines.FindJumpSpline` (`/Game/Blueprints/Libraries/BPFL_GlobalData.ToWorldPosition` (`local.StartLocation`)) (`/Game/Blueprints/Libraries/BPFL_GlobalData.ToWorldPosition` (`local.DestinationLocation`)) 0.65 _jumpspline))
                      (if _success
                        (bind (_hit _ishit_) (`/Game/Blueprints/Libraries/BPFL_Splines.SplineTraceByChannel` _jumpspline 1.0 "TraceTypeQuery3"))
                        (if _ishit_
                          (goto _label_3 :!via `Continue`)
                          (else
                            ;; Determine if is hard fall
                            (if (not (> (+ (`local.FallDistance`) (`local.VerticalTravel`)) 0.0))
                              (set `local.isHardLanding` true)
                              (set `local.HazardAccumulator` (+ (`local.HazardAccumulator`) 50)))
                            ;; Determine if Hop
                            (if (and (<= (`local.HorizontalTravel`) 1.5) (> 1.5 (`local.VerticalTravel`)))
                              (set `local.CurrentMoveType` "NewEnumerator1")
                              (else
                                ;; Determine if Long Jump
                                (if (>= (`local.HorizontalTravel`) (`local.VerticalTravel`))
                                  (set `local.CurrentMoveType` "NewEnumerator2")
                                  (else
                                    ;; Determine if High Jump
                                    (if (< (`local.HorizontalTravel`) (`local.VerticalTravel`))
                                      (set `local.CurrentMoveType` "NewEnumerator3")
                                      (else
                                        ;; Determine if Fall
                                        (if (< (`local.HorizontalTravel`) (* (`local.VerticalTravel`) -1.0))
                                          (set `local.CurrentMoveType` "NewEnumerator4")
                                          (else
                                            (goto _label_3 :!via `Continue`)))))))))))
                        (else
                          (goto _label_3 :!via `Continue`)))
                      (else
                        (goto _label_3 :!via `Continue`)))
                    (else
                      (set `local.CurrentMoveType` "NewEnumerator0")))
                  ;; Add move
                  (`KismetArrayLibrary.Array_Add` (`local.Possible Moves`) (make `/Game/Data/AI/F_MoveData` (`local.DestinationWorldLocation`) (`local.MoveCost`) (`local.CurrentMoveType`) (`local.CurrentDirection`) (`local.isHardLanding`) _startedgeheight _destinationnearedgeheightheight _destinationfaredgeheight (`local.HazardAccumulator`) (`local.HorizontalTravel`) (`local.VerticalTravel`)))
                  (goto _label_3 :!via `Continue`)
                  (else
                    (goto _label_3 :!via `Continue`))))
              (:`Completed`
                (goto _label_2 :!via `Continue`))))
          (:`Complete`
            (goto _label :!via `Continue`))))
      (:`Completed`
        ;[0 1 0 0.5] DONE!
        (return (`local.Possible Moves`))))
    (else
      ;[1.472 1.344 -0.602 0.5] quit if current position invalid
      (`KismetSystemLibrary.PrintString` "Currently not in valid location!")
      (return (`local.Possible Moves`)))))

(fn `FindNodes`
  (params (Position :type "/Game/Blueprints/Libraries/F_IntVector2d Structure"))
  (returns (TacticalNodes :type "Map of IntVector Structure to /Game/Data/AI/F_TacticalNode Structure"))
  (locals (OutputNodes :type "Map of IntVector Structure to /Game/Data/AI/F_TacticalNode Structure"))
  (bind (_x _y) (break `/Game/Blueprints/Libraries/F_IntVector2d` Position))
  (bind (_value _returnvalue) (`BlueprintMapLibrary.Map_Find` (`self.NavigablePoints`) Position))
  (bind _nodes (break `/Game/Data/AI/F_TacticalArray` _value))
  (`BlueprintMapLibrary.Map_Clear` (`local.OutputNodes`))
  (if _returnvalue
    (bind _keys (`BlueprintMapLibrary.Map_Keys` _nodes))
    (bind _arrayelement (`/Game/Blueprints/Libraries/BPML_Utilities.ForEachLoop_Real` _keys :!label _label)
      (:`LoopBody`
        (bind (_value_2 _returnvalue_2) (`BlueprintMapLibrary.Map_Find` _nodes _arrayelement))
        (if _returnvalue_2
          (`BlueprintMapLibrary.Map_Add` (`local.OutputNodes`) (make `IntVector` _x _y _arrayelement) _value_2)
          (goto _label :!via `Continue`)
          (else
            (goto _label :!via `Continue`))))
      (:`Completed`
        _)))
  (return (`local.OutputNodes`)))

(fn `GetNearbyChebyshev`
  (params (Start :type "IntVector Structure") (Distance :type Integer))
  (returns (Nearby :type "Array of IntVector Structure"))
  (locals (Neighbors :type "Array of IntVector Structure"))
  (bind (_x _y) (break `IntVector` Start))
  (bind _keys (`BlueprintMapLibrary.Map_Keys` (`self.NavigablePoints`)))
  (bind _arrayelement (`/Game/Blueprints/Libraries/BPML_Utilities.ForEachLoop_Real` _keys :!label _label)
    (:`LoopBody`
      (if (> (`/Game/Blueprints/Libraries/BPML_VectorMath.ChebyshevDistance (2d)` _arrayelement (make `/Game/Blueprints/Libraries/F_IntVector2d` _x _y)) Distance)
        (goto _label :!via `Continue`)
        (else
          (bind (_value _returnvalue) (`BlueprintMapLibrary.Map_Find` (`self.NavigablePoints`) _arrayelement))
          (if _returnvalue
            (bind _keys_2 (`BlueprintMapLibrary.Map_Keys` (`.Nodes_9_ADB601575A484309BE75B222EA95378A` (break `/Game/Data/AI/F_TacticalArray` _value))))
            (bind _arrayelement_2 (`/Game/Blueprints/Libraries/BPML_Utilities.ForEachLoop_Real` _keys_2 :!label _label_2)
              (:`LoopBody`
                (bind (_x_2 _y_2) (break `/Game/Blueprints/Libraries/F_IntVector2d` _arrayelement))
                (bind _intvector (make `IntVector` _x_2 _y_2 _arrayelement_2))
                (if (> (`/Game/Blueprints/Libraries/BPML_VectorMath.ChebyshevDistance (IntVector)` (`local.Start`) _intvector) Distance)
                  (goto _label_2 :!via `Continue`)
                  (else
                    (`KismetArrayLibrary.Array_Add` (`local.Neighbors`) _intvector)
                    (goto _label_2 :!via `Continue`))))
              (:`Completed`
                (goto _label :!via `Continue`)))
            (else
              (goto _label :!via `Continue`))))))
    (:`Completed`
      (return (`local.Neighbors`)))))

(fn `GetNearbyEuclidean`
  (params (Start :type "IntVector Structure") (Distance :type Integer))
  (returns (Nearby :type "Array of IntVector Structure"))
  (locals (Neighbors :type "Array of IntVector Structure"))
  (bind (_x _y) (break `IntVector` Start))
  (bind _keys (`BlueprintMapLibrary.Map_Keys` (`self.NavigablePoints`)))
  (bind _arrayelement (`/Game/Blueprints/Libraries/BPML_Utilities.ForEachLoop_Real` _keys :!label _label)
    (:`LoopBody`
      (if (> (`/Game/Blueprints/Libraries/BPML_VectorMath.EuclideanDistance (2d)` _arrayelement (make `/Game/Blueprints/Libraries/F_IntVector2d` _x _y)) Distance)
        (goto _label :!via `Continue`)
        (else
          (bind (_value _returnvalue) (`BlueprintMapLibrary.Map_Find` (`self.NavigablePoints`) _arrayelement))
          (if _returnvalue
            (bind _keys_2 (`BlueprintMapLibrary.Map_Keys` (`.Nodes_9_ADB601575A484309BE75B222EA95378A` (break `/Game/Data/AI/F_TacticalArray` _value))))
            (bind _arrayelement_2 (`/Game/Blueprints/Libraries/BPML_Utilities.ForEachLoop_Real` _keys_2 :!label _label_2)
              (:`LoopBody`
                (bind (_x_2 _y_2) (break `/Game/Blueprints/Libraries/F_IntVector2d` _arrayelement))
                (bind _intvector (make `IntVector` _x_2 _y_2 _arrayelement_2))
                (if (> (`/Game/Blueprints/Libraries/BPML_VectorMath.EuclideanDistance (IntVector)` (`local.Start`) _intvector) Distance)
                  (goto _label_2 :!via `Continue`)
                  (else
                    (`KismetArrayLibrary.Array_Add` (`local.Neighbors`) _intvector)
                    (goto _label_2 :!via `Continue`))))
              (:`Completed`
                (goto _label :!via `Continue`)))
            (else
              (goto _label :!via `Continue`))))))
    (:`Completed`
      (return (`local.Neighbors`)))))

(fn `GetNearbyManhatten`
  (params (Start :type "IntVector Structure") (Distance :type Integer))
  (returns (Nearby :type "Array of IntVector Structure"))
  (locals (Neighbors :type "Array of IntVector Structure"))
  (bind (_x _y) (break `IntVector` Start))
  (bind _keys (`BlueprintMapLibrary.Map_Keys` (`self.NavigablePoints`)))
  (bind _arrayelement (`/Game/Blueprints/Libraries/BPML_Utilities.ForEachLoop_Real` _keys :!label _label)
    (:`LoopBody`
      (if (> (`/Game/Blueprints/Libraries/BPML_VectorMath.ManhattenDistance (2d)` _arrayelement (make `/Game/Blueprints/Libraries/F_IntVector2d` _x _y)) Distance)
        (goto _label :!via `Continue`)
        (else
          (bind (_value _returnvalue) (`BlueprintMapLibrary.Map_Find` (`self.NavigablePoints`) _arrayelement))
          (if _returnvalue
            (bind _keys_2 (`BlueprintMapLibrary.Map_Keys` (`.Nodes_9_ADB601575A484309BE75B222EA95378A` (break `/Game/Data/AI/F_TacticalArray` _value))))
            (bind _arrayelement_2 (`/Game/Blueprints/Libraries/BPML_Utilities.ForEachLoop_Real` _keys_2 :!label _label_2)
              (:`LoopBody`
                (bind (_x_2 _y_2) (break `/Game/Blueprints/Libraries/F_IntVector2d` _arrayelement))
                (bind _intvector (make `IntVector` _x_2 _y_2 _arrayelement_2))
                (if (> (`/Game/Blueprints/Libraries/BPML_VectorMath.ManhattenDistance (IntVector)` (`local.Start`) _intvector) Distance)
                  (goto _label_2 :!via `Continue`)
                  (else
                    (`KismetArrayLibrary.Array_Add` (`local.Neighbors`) _intvector)
                    (goto _label_2 :!via `Continue`))))
              (:`Completed`
                (goto _label :!via `Continue`)))
            (else
              (goto _label :!via `Continue`))))))
    (:`Completed`
      (return (`local.Neighbors`)))))

(fn `GetNode`
  (params (Position :type "IntVector Structure"))
  (returns (FoundNode :type "/Game/Data/AI/F_TacticalNode Structure") (isFound :type Boolean))
  (bind (_value _returnvalue) (`BlueprintMapLibrary.Map_Find` (`self.NavigablePoints`) (make `/Game/Blueprints/Libraries/F_IntVector2d` Position_X Position_Y)))
  (bind (_value_2 _returnvalue_2) (`BlueprintMapLibrary.Map_Find` (break `/Game/Data/AI/F_TacticalArray` _value) Position_Z))
  (return _value_2 (and _returnvalue_2 _returnvalue)))

(fn `GetPositionAtTile`
  (params (Input :type "/Game/Blueprints/Libraries/F_IntVector2d Structure"))
  (returns (WorldPosition :type "IntVector Structure") (TileCoordinate :type "IntVector Structure"))
  (bind (_value _returnvalue) (`BlueprintMapLibrary.Map_Find` (`self.NavigablePoints`) (make `/Game/Blueprints/Libraries/F_IntVector2d` Input_x_4_5DF768701C18439E990D97A68C679FD1 Input_y_5_7BC2096791B1495487AD3F10E7364099)))
  (bind _nodes (break `/Game/Data/AI/F_TacticalArray` _value))
  (if _returnvalue
    (bind _keys (`BlueprintMapLibrary.Map_Keys` _nodes))
    (bind (_indexofmaxvalue _maxvalue) (`KismetMathLibrary.MaxOfIntArray` _keys))
    (bind _intvector (make `IntVector` Input_x_4_5DF768701C18439E990D97A68C679FD1 Input_y_5_7BC2096791B1495487AD3F10E7364099 _maxvalue))
    (bind (_value_2 _returnvalue_2) (`BlueprintMapLibrary.Map_Find` _nodes _maxvalue))
    (return (`/Game/Blueprints/Libraries/BPML_VectorMath.Add (IntVector)` (`/Game/Blueprints/Libraries/BPML_VectorMath.Multiply (IntVector)` _intvector (make `IntVector` 100 100 100)) (make `IntVector` 0 0 (select `bool` _returnvalue_2 :`true` (`.UnitHeight_20_E95CDC97603540709376EEFBAD8A3F15` (break `/Game/Data/AI/F_TacticalNode` _value_2))))) _intvector)))

(fn `GetSize`
  (returns (Size :type Integer))
  (locals (NumNodes :type Integer))
  (bind _navigablepoints (`self.NavigablePoints`))
  (set `local.NumNodes` 0)
  (bind _keys (`BlueprintMapLibrary.Map_Keys` _navigablepoints))
  (bind _arrayelement (`/Game/Blueprints/Libraries/BPML_Utilities.ForEachLoop_Real` _keys :!label _label)
    (:`LoopBody`
      (bind (_value _returnvalue) (`BlueprintMapLibrary.Map_Find` _navigablepoints _arrayelement))
      (if _returnvalue
        (set `local.NumNodes` (+ (`BlueprintMapLibrary.Map_Length` (break `/Game/Data/AI/F_TacticalArray` _value)) (`local.NumNodes`)))
        (goto _label :!via `Continue`)
        (else
          (goto _label :!via `Continue`))))
    (:`Completed`
      (return (`local.NumNodes`)))))

(fn `SetOccupiedAt`
  (params (Location :type "IntVector Structure"))
  (returns (Success :type Boolean))
  (bind (_foundnode _isfound) (`self.GetNode` Location))
  (if _isfound
    (bind (_position _terraintype _occupied _unit _pickups _unitheight _northedgeheight _eastedgeheight _southedgeheight _westedgeheight) (break `/Game/Data/AI/F_TacticalNode` _foundnode))
    (`self.AddNode` (make `/Game/Data/AI/F_TacticalNode` _position _terraintype true _unit _pickups _unitheight _northedgeheight _eastedgeheight _southedgeheight _westedgeheight) Location)
    (return true)
    (else
      (return false))))

(fn `UserConstructionScript`)