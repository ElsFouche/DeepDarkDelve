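; Base AI controller for tactical grid units that picks a target when its unit's turn starts.
; It caches the controlled BP_BaseUnit and the game state's tactical cortex, which an update event refreshes.
; On turn start it gathers all units on tiles within move and jump range, unfiltered by team, and targets the lowest-health one.
; It only stores the target; no move or attack follows.
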(event `self.ReceiveBeginPlay`
  ; Begin Play
  (bind _tacticalcortex (message `/Game/Blueprints/Interfaces/BPI_GameStateCombat.GetTacticalCortex` (`GameplayStatics.GetGameState`)))
  (set `self.TacticalCortex` _tacticalcortex)
  (bind (_asbp_base_unit _success) (`self.GetControlledUnit`))
  (if _success
    (set `self.ControlledUnit` _asbp_base_unit)))

(event `/Game/Blueprints/Interfaces/BPI_GameStateCombat.TacticalCortexUpdated`
  (params (CompleteTacticalCortex :type "/Game/Blueprints/Units/AI/BP_TacticalCortex Object Reference (by ref)"))
  (set `self.TacticalCortex` CompleteTacticalCortex))

(event `/Game/Blueprints/Interfaces/BPI_GameStateCombat.StartUnitTurn`
  (bind _unitsinrange (`self.GetUnitsInRange`))
  (bind _output_get (set `self.Units in Range` _unitsinrange))
  (bind _unitatlowesthp (`self.GetUnitAtLowestHP` _output_get))
  (set `self.Target` _unitatlowesthp))

(fn `GetAllUnits`
  (returns (AllUnits :type "Array of /Game/Blueprints/Units/BP_BaseUnit Object Reference"))
  (return))

(fn `GetControlledUnit`
  (returns (`AsBP Base Unit` :type "/Game/Blueprints/Units/BP_BaseUnit Object Reference") (Success :type Boolean))
  (bind _asbp_base_unit (cast `/Game/Blueprints/Units/BP_BaseUnit` (`self.K2_GetPawn`))
    (:`then`
      (return _asbp_base_unit true))
    (:`CastFailed`
      (return null false))))

(fn `GetTacticalCortex`
  (returns (TacticalCortex :type "/Game/Blueprints/Units/AI/BP_TacticalCortex Object Reference"))
  (return null))

(fn `GetUnitAtLowestHP`
  (params (Units :type "Array of /Game/Blueprints/Units/BP_BaseUnit Object Reference"))
  (returns (UnitAtLowestHP :type "/Game/Blueprints/Units/BP_BaseUnit Object Reference"))
  (locals (LowestHPUnit :type "/Game/Blueprints/Units/BP_BaseUnit Object Reference"))
  (for _array_element Units
    (bind _lowesthpunit (`local.LowestHPUnit`)
      (:`then`
        (if (< (`.Health_29_D64E61F44D0663E97EE38B85A4EEBC31` (break `/Game/Data/Unit/F_UnitStats` (`/Game/Blueprints/Units/BP_BaseUnit.CurrStats` _array_element))) (`.Health_29_D64E61F44D0663E97EE38B85A4EEBC31` (break `/Game/Data/Unit/F_UnitStats` (`/Game/Blueprints/Units/BP_BaseUnit.CurrStats` _lowesthpunit))))
          (set `local.LowestHPUnit` _array_element :!label _label)))
      (:`else`
        (goto _label))))
  (return (`local.LowestHPUnit`)))

(fn `GetUnitsInRange`
  (returns (UnitsInRange :type "Array of /Game/Blueprints/Units/BP_BaseUnit Object Reference"))
  (locals (TilesInRange :type "Array of IntVector Structure") (Units :type "Array of /Game/Blueprints/Units/BP_BaseUnit Object Reference"))
  (bind _controlledunit (`self.ControlledUnit`))
  (bind ((`Move_18_01D06AB942472614BDB3F491D217C085` _move) (`Jump_19_4BDD3D614ABF55D5A43C52ACFF31CA3C` _jump)) (break `/Game/Data/Unit/F_UnitStats` (`/Game/Blueprints/Units/BP_BaseUnit.CurrStats` _controlledunit)))
  (set `local.TilesInRange` (`/Game/Blueprints/ActorComponents/AC_GridNavigation.GetTilesInMoveRange` (`/Game/Blueprints/Units/BP_BaseUnit.AC_GridNavigation` _controlledunit) (`/Game/Blueprints/Libraries/BPFL_GlobalData.VectToTile` (`self.K2_GetActorLocation` _controlledunit)) _move _jump))
  (bind _allunits (message `/Game/Blueprints/Interfaces/BPI_GameStateCombat.GetAllUnits` (`GameplayStatics.GetGameState`)))
  (for _array_element _allunits
    (if (`KismetArrayLibrary.Array_Contains` (`local.TilesInRange`) (`/Game/Blueprints/Libraries/BPFL_GlobalData.VectToTile` (`self.K2_GetActorLocation` _array_element)))
      (`KismetArrayLibrary.Array_Add` (`local.Units`) _array_element)))
  (return (`local.Units`)))

(fn `UserConstructionScript`)