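; Blueprint function library of procedural-generation helpers for shuffled index orderings, grid neighbor queries and tile lookups.
; Get2dNeighbors gathers up to eight unique flat-index neighbors with optional per-axis wrapping.
; GetNeighbor offsets a 3D position using modulo, returning a placeholder vector and IsWrapped flag when out of bounds without Wrap.
; GetRelevantTileInfo joins a tile map entry with DT_TileShapeInfo traits, defaulting to non-standable air when either lookup fails.
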(fn `GenerateShuffledOrdering`
  (params (maximum :type Integer :default 51))
  (returns (shuffled :type "Array of Integer"))
  (locals (Return :type "Array of Integer"))
  (bind _return (`local.Return`))
  (for _index (range (+ maximum 1))
    (`KismetArrayLibrary.Array_Add` _return _index))
  (`KismetArrayLibrary.Array_Shuffle` _return)
  (return _return))

(fn `Get2dNeighbors`
  (params (Dimensions :type "IntVector Structure") (Index :type Integer) (wrapX :type Boolean) (wrapY :type Boolean))
  (returns (NeighborIndices :type "Array of Integer"))
  (locals (Neighbors :type "Array of Integer") (isNotTop :type Boolean) (isNotLeft :type Boolean) (isNotRight :type Boolean) (isNotBottom :type Boolean))
  (bind _x (break `IntVector` Dimensions))
  (bind (_x_2 _y) (break `IntVector` Dimensions))
  (bind (_x_3 _y_2) (break `IntVector` Dimensions))
  (bind (_x_4 _y_3) (break `IntVector` Dimensions))
  (bind _x_5 (break `IntVector` Dimensions))
  (bind (_x_6 _y_4) (break `IntVector` Dimensions))
  (bind (_x_7 _y_5) (break `IntVector` Dimensions))
  (bind (_x_8 _y_6) (break `IntVector` Dimensions))
  (bind (_x_9 _y_7) (break `IntVector` Dimensions))
  (bind _position (`/Game/Blueprints/Libraries/BPML_3dArray.GetPositionFromIndex` Dimensions Index))
  (bind _neighbors (`local.Neighbors`))
  (bind (_x_10 _y_8) (break `IntVector` _position))
  (bind (_x_11 _y_9) (break `IntVector` _position))
  (bind (_x_12 _y_10) (break `IntVector` _position))
  (bind (_x_13 _y_11) (break `IntVector` _position))
  (bind (_x_14 _y_12) (break `IntVector` _position))
  (bind (_x_15 _y_13) (break `IntVector` _position))
  (bind (_x_16 _y_14) (break `IntVector` _position))
  (bind (_x_17 _y_15) (break `IntVector` _position))
  (bind (_x_18 _y_16) (break `IntVector` _position))
  ; Determine if on any edges
  (set `local.isNotBottom` (> _y_16 0))
  (set `local.isNotRight` (< _x_18 _x_9))
  (set `local.isNotLeft` (> _x_18 0))
  (set `local.isNotTop` (< _y_16 _y_7))
  ; Top Left
  (if (and (or (`local.isNotLeft`) wrapX) (or wrapY (`local.isNotTop`)))
    (`KismetArrayLibrary.Array_AddUnique` (`local.Neighbors`) (`/Game/Blueprints/Libraries/BPML_3dArray.GetIndexFromPosition` (make `IntVector` (mod (+ (- _x_15 1) _x_6) _x_6) (mod (+ (+ _y_13 1) _y_4) _y_4)) Dimensions)))
  ; Top
  (if (or wrapY (`local.isNotTop`))
    (`KismetArrayLibrary.Array_AddUnique` (`local.Neighbors`) (`/Game/Blueprints/Libraries/BPML_3dArray.GetIndexFromPosition` (make `IntVector` _x_16 (mod (+ (+ _y_14 1) _y_5) _y_5)) Dimensions)))
  ; Top Right
  (if (and (or (`local.isNotRight`) wrapX) (or wrapY (`local.isNotTop`)))
    (`KismetArrayLibrary.Array_AddUnique` (`local.Neighbors`) (`/Game/Blueprints/Libraries/BPML_3dArray.GetIndexFromPosition` (make `IntVector` (mod (+ (+ _x_17 1) _x_8) _x_8) (mod (+ (+ _y_15 1) _y_6) _y_6)) Dimensions)))
  ; Left
  (if (or (`local.isNotLeft`) wrapX)
    (`KismetArrayLibrary.Array_AddUnique` (`local.Neighbors`) (`/Game/Blueprints/Libraries/BPML_3dArray.GetIndexFromPosition` (make `IntVector` (mod (+ (- _x_14 1) _x_5) _x_5) _y_12) Dimensions)))
  ; Right
  (if (or (`local.isNotRight`) wrapX)
    (`KismetArrayLibrary.Array_AddUnique` (`local.Neighbors`) (`/Game/Blueprints/Libraries/BPML_3dArray.GetIndexFromPosition` (make `IntVector` (mod (+ (+ _x_10 1) _x) _x) _y_8) Dimensions)))
  ; Bottom Left
  (if (and (or (`local.isNotLeft`) wrapX) (or wrapY (`local.isNotBottom`)))
    (`KismetArrayLibrary.Array_AddUnique` (`local.Neighbors`) (`/Game/Blueprints/Libraries/BPML_3dArray.GetIndexFromPosition` (make `IntVector` (mod (+ (- _x_11 1) _x_2) _x_2) (mod (+ (- _y_9 1) _y) _y)) Dimensions)))
  ; Bottom
  (if (or wrapY (`local.isNotBottom`))
    (`KismetArrayLibrary.Array_AddUnique` (`local.Neighbors`) (`/Game/Blueprints/Libraries/BPML_3dArray.GetIndexFromPosition` (make `IntVector` _x_12 (mod (+ (- _y_10 1) _y_2) _y_2)) Dimensions)))
  ; Bottom Right
  (if (and (or (`local.isNotRight`) wrapX) (or wrapY (`local.isNotBottom`)))
    (`KismetArrayLibrary.Array_AddUnique` (`local.Neighbors`) (`/Game/Blueprints/Libraries/BPML_3dArray.GetIndexFromPosition` (make `IntVector` (mod (+ (+ _x_13 1) _x_4) _x_4) (mod (+ (- _y_11 1) _y_3) _y_3)) Dimensions)))
  (`KismetArrayLibrary.Array_RemoveItem` _neighbors Index)
  (return _neighbors))

(fn `GetNeighbor`
  (params (Dimensions :type "IntVector Structure") (Position :type "IntVector Structure") (Offset :type "IntVector Structure") (Wrap :type Boolean))
  (returns (Neighbor :type "IntVector Structure") (isWrapped :type Boolean))
  (bind (_x _y _z) (break `IntVector` Dimensions))
  (bind ____ (`/Game/Blueprints/Libraries/BPML_VectorMath.Add (IntVector)` Position Offset))
  (bind (_x_2 _y_2 _z_2) (break `IntVector` ____))
  (bind (_x_3 _y_3 _z_3) (break `IntVector` (`/Game/Blueprints/Libraries/BPML_VectorMath.Modulo (IntVector)` (`/Game/Blueprints/Libraries/BPML_VectorMath.Add (IntVector)` Dimensions ____) Dimensions)))
  (bind _returnvalue (or (not (or (> _x_2 _x) (> _y_2 _y) (> _z_2 _z) (< _x_2 0) (< _y_2 0) (< _z_2 0))) Wrap))
  (return (make `IntVector` (`KismetMathLibrary.SelectInt` _x_3 4 _returnvalue) (`KismetMathLibrary.SelectInt` _y_3 20 _returnvalue) (`KismetMathLibrary.SelectInt` _z_3 69 _returnvalue)) (not _returnvalue)))

(fn `GetRelevantTileInfo`
  (params (TileInfo :type "Map of IntVector Structure to /Game/Data/Procedural/F_TileInfo Structure (by ref)") (Position :type "IntVector Structure (by ref)") (__WorldContext :type "Object Object Reference"))
  (returns (isStandable :type Boolean) (isTopAir :type Boolean) (isBottomAir :type Boolean) (TileShape :type "/Game/Data/Procedural/E_TileShapes Enum") (TerrainType :type "/Game/Data/Procedural/E_TerrainTypes Enum") (CharacterHeight :type Integer))
  (bind (_value _returnvalue) (`BlueprintMapLibrary.Map_Find` TileInfo Position))
  (bind ((`TerrainType_11_5936953DBE95436486B99445F991EACC` _terraintype) (`TileShape_27_3B868F91D0354B07A771A75B225AB195` _tileshape)) (break `/Game/Data/Procedural/F_TileInfo` _value))
  (if _returnvalue
    (bind _returnvalue_2 (`|GetDataTableRow` "/Game/Data/Procedural/DT_TileShapeInfo.DT_TileShapeInfo" (`KismetStringLibrary.Conv_StringToName` (`|GetEnumeratorNameAsString` _tileshape)))
      (:`then`
        (bind ((`isStandable_22_456497ED2A94426993A4C13968E66FF4` _isstandable) (`CharacterHeight_7_BE088372A2EA429190A7AF61BF144925` _characterheight) (`isTopAir_29_14D208A27D7E4CC8976B7963B55A664B` _istopair) (`isBottomAir_30_11D4C03093B741B4ABCB9ECDDF464730` _isbottomair)) (break `/Game/Data/Procedural/F_TileShapeInfo` _returnvalue_2))
        (return _isstandable _istopair _isbottomair _tileshape _terraintype _characterheight))
      (:`RowNotFound`
        _)))
  (return false true true "NewEnumerator29" "NewEnumerator0" 0))