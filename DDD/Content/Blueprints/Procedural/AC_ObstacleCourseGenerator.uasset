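; Obstacle course generator component that procedurally builds tile-based room terrain and returns parsed level data to the requester.
; GenerateRoomStart randomizes grid corner heights, then iteratively reduces neighbor constraint failures using shuffled local search, capped by MaxSmoothingLoops.
; Corner heights become stacked tiles with shaped, rotated tops over an air fill, with work spread across ticks.
; It then sprinkles a random prebuilt, sets four edge-midpoint entrances and parses the level info.
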(event EventBeginPlay
  (|CallParentFunction) ; This node is disabled and will not be called.\nDrag off pins to build functionality.
)

(event EventTick
  (params (DeltaSeconds :type Float%20%28single-precision%29))
  (|CallParentFunction DeltaSeconds) ; This node is disabled and will not be called.\nDrag off pins to build functionality.
)

(event EventGetParsedData
  (params (PCGData :type F%20PCG%20Data%20Structure) (TacticalCortex :type BP%20Tactical%20Cortex%20Object%20Reference) (SpawnPoints :type Array%20of%20F%20Unit%20Spawn%20Point%20Structures))
  ;[-1.018 119 -1.043 0.5] DONE
  (Class|BPIRoomConstruction|LevelDataComplete(Message) (stale EventGenerateRoomStart RequestedBy) PCGData TacticalCortex SpawnPoints))

(event EventGenerateRoomStart
  (params (RequestedBy :type Object%20Object%20Reference%20%28by%20ref%29) (RoomType :type E_RoomTypes%20Enum :default "NewEnumerator0") (RoomDimensions :type Int%20Vector%20Structure))
  (bind ____ (Utilities|Add(IntVector) RoomDimensions (Utilities|Struct|MakeIntVector 1 1 0)))
  (bind _array (Utilities|Array|MakeArray "NewEnumerator1"))
  (bind _cornermap (Variables|Default|GetCornerMap))
  (bind _levelinfo (Variables|Default|GetLevelInfo))
  (bind _heightstocheck (Variables|Default|GetHeightsToCheck))
  (bind (_dimensions _entrances) (Utilities|Struct|BreakF_LevelInfo _levelinfo))
  (bind (_x _y) (Utilities|Struct|BreakIntVector _dimensions))
  (bind _____2 (Utilities|Scale(IntVector) _dimensions 0.5))
  ;[0.15 0.15 0.15 0.5] generate array of valid heights
  (Variables|Default|SetDimensions RoomDimensions)
  (bind _index (Utilities|ForLoopReal 0 (Math|Integer|Min(Integer) (.Z (Utilities|Struct|BreakIntVector RoomDimensions)) 8) :!label _label)
    (:LoopBody
      (Utilities|Array|SetArrayElem (Variables|Default|GetHeightsToCheck) _index _index true)
      (goto _label Continue))
    (:Complete
      ;[0.15 0.15 0.15 0.5] initialize cell corners at random valid heights
      (bind _index_2 (Utilities|ForLoopReal 0 (.x ____) :!label _label_2)
        (:LoopBody
          (bind _index_3 (Utilities|ForLoopReal 0 (.y ____) :!label _label_3)
            (:LoopBody
              (Utilities|Map|Add (Variables|Default|GetCornerMap) (Utilities|Struct|MakeF_IntVector2d _index_2 _index_3) (.OutItem (Utilities|Array|Random (Variables|Default|GetHeightsToCheck))))
              (goto _label_3 Continue))
            (:Complete
              (goto _label_2 Continue))))
        (:Complete
          (Variables|Default|SetNumSmoothingLoops 0)
          (bind _keys (Utilities|Map|Keys (Variables|Default|GetCornerMap) :!label _label_4))
          (Utilities|Array|Shuffle _keys)
          (Variables|Default|SetisTweaked false)
          ;[0.15 0.15 0.15 0.5 32] for each corner, if its height doesn't vibe with its neighbors', try other heights until you get something better. if you do change a height, make a note.
          (bind _arrayelement (Utilities|ForEachLoopReal _keys :!label _label_5)
            (:LoopBody
              (bind ___ (CallFunction|TallyConstraintFailures _arrayelement (.Value (Utilities|Map|Find (Variables|Default|GetCornerMap) _arrayelement))))
              (if (> ___ 0)
                (Variables|Default|SetBestHeightSoFar (.Value (Utilities|Map|Find (Variables|Default|GetCornerMap) _arrayelement)))
                (Variables|Default|SetLeastErrors ___)
                (Utilities|Array|Shuffle _heightstocheck)
                (bind _arrayelement_2 (Utilities|ForEachLoopReal _heightstocheck :!label _label_6)
                  (:LoopBody
                    (bind ____2 (CallFunction|TallyConstraintFailures _arrayelement _arrayelement_2))
                    (if (and (< ____2 (Variables|Default|GetLeastErrors)) (!= ____2 (.Value (Utilities|Map|Find (Variables|Default|GetCornerMap) _arrayelement))))
                      (bind _output_get (Variables|Default|SetLeastErrors ____2))
                      (bind _output_get_2 (Variables|Default|SetBestHeightSoFar _arrayelement_2))
                      (Variables|Default|SetisTweaked true)
                      (goto _label_6 Continue)
                      (else
                        (goto _label_6 Continue))))
                  (:Completed
                    (if (== (Variables|Default|GetBestHeightSoFar) (.Value (Utilities|Map|Find (Variables|Default|GetCornerMap) _arrayelement)))
                      (goto _label_5 Continue)
                      (else
                        (Utilities|Map|Add (Variables|Default|GetCornerMap) _arrayelement (Variables|Default|GetBestHeightSoFar))
                        (goto _label_5 Continue)))))
                (else
                  (goto _label_5 Continue))))
            (:Completed
              ;[0.15 0.15 0.15 0.5] run it again if we made any edits last time, and we haven't hit our loop limit
              (if (Variables|Default|GetisTweaked)
                (Math|Integer|IncrementInt (Variables|Default|GetNumSmoothingLoops)
                  (:%20%20
                    (if (<= (Variables|Default|GetNumSmoothingLoops) (Variables|Default|GetMaxSmoothingLoops))
                      (Utilities|FlowControl|DelayUntilNextTick)
                      (goto _label_4)
                      (else
                        _)))))
              ;[0.15 0.15 0.15 0.5] fill level info with air tiles first
              (bind _index_4 (Utilities|ForRealLoop(3d) (Utilities|Struct|MakeIntVector 0 0 0) (Variables|Default|GetDimensions) :!label _label_7)
                (:LoopBody
                  (CallFunction|AddTile _index_4 "NewEnumerator0" "NewEnumerator0" "NewEnumerator29" "NewEnumerator0")
                  (goto _label_7 Continue))
                (:Complete
                  ;[0.15 0.15 0.15 0.5] Get Top Tile Info for each cell from corner heights
                  (bind _index_5 (Utilities|ForLoopReal 0 (.y (Utilities|Struct|BreakF_IntVector2d (Utilities|ToIntVector2d (Variables|Default|GetDimensions)))) :!label _label_8)
                    (:LoopBody
                      (Utilities|FlowControl|DelayUntilNextTick)
                      (bind _index_6 (Utilities|ForLoopReal 0 (.x (Utilities|Struct|BreakF_IntVector2d (Utilities|ToIntVector2d (Variables|Default|GetDimensions)))) :!label _label_9)
                        (:LoopBody
                          (Utilities|FlowControl|DelayUntilNextTick)
                          (bind (_tileshape _rotation _height) (CallFunction|GetTileInfofromHeights (.Value (Utilities|Map|Find _cornermap (Utilities|Struct|MakeF_IntVector2d (+ _index_6 1) (+ _index_5 1)))) (.Value (Utilities|Map|Find _cornermap (Utilities|Struct|MakeF_IntVector2d _index_6 (+ _index_5 1)))) (.Value (Utilities|Map|Find _cornermap (Utilities|Struct|MakeF_IntVector2d _index_6 _index_5))) (.Value (Utilities|Map|Find _cornermap (Utilities|Struct|MakeF_IntVector2d (+ _index_6 1) _index_5))) true))
                          ;[0.15 0.15 0.15 0.5] add tiles to level info
                          (bind _index_7 (Utilities|ForLoopReal 0 (- _height 1) :!label _label_10)
                            (:LoopBody
                              (CallFunction|AddTile (Utilities|Struct|MakeIntVector _index_6 _index_5 _index_7) "NewEnumerator1" "NewEnumerator0" "NewEnumerator0" _array)
                              (goto _label_10 Continue))
                            (:Complete
                              (CallFunction|AddTile (Utilities|Struct|MakeIntVector _index_6 _index_5 _height) "NewEnumerator1" _rotation _tileshape _array)
                              (Development|PrintString (Utilities|String|Append "tile added at " (Utilities|String|ToString(Integer) (Utilities|Struct|MakeIntVector _index_6 _index_5 _height))))
                              (goto _label_9 Continue))))
                        (:Complete
                          (goto _label_8 Continue))))
                    (:Complete
                      ;[0.15 0.15 0.15 0.5] Sprinkle with Tile Prebuilts
                      (bind _outrownames (DataTable|GetDataTableRowNames "/Game/Data/Procedural/DT_TilePrebuilts.DT_TilePrebuilts"))
                      (bind _output_get_3 (Variables|Default|SetChosenPrebuilt (.OutItem (Utilities|Array|Random _outrownames))))
                      (CallFunction|SprinkleTilePrebuilts _output_get_3)
                      ;[0.15 0.15 0.15 0.5] calculate entrances
                      (Utilities|Array|SetArrayElem _entrances 0 (Utilities|Struct|MakeIntVector (.x _____2) 0 (.z _____2)) true)
                      (Utilities|Array|SetArrayElem _entrances 1 (Utilities|Struct|MakeIntVector 0 (.y _____2) (.z _____2)) true)
                      (Utilities|Array|SetArrayElem _entrances 2 (Utilities|Struct|MakeIntVector (.x _____2) _y (.z _____2)) true)
                      (Utilities|Array|SetArrayElem _entrances 3 (Utilities|Struct|MakeIntVector _x (.y _____2) (.z _____2)) true)
                      ;[-1.018 119 -1.043 0.5] DONE
                      (CallFunction|ParseLevelInfo (Variables|Default|GetLevelInfo)))))))))))))

(fn TallyConstraintFailures
  (params (CurrentCorner :type F%20Int%20Vector%202d%20Structure) (TestHeight :type Integer))
  (bind ____ (Utilities|Add(IntVector2d) CurrentCorner (Utilities|Struct|MakeF_IntVector2d -1 1)))
  (bind _____2 (Utilities|Add(IntVector2d) CurrentCorner (Utilities|Struct|MakeF_IntVector2d -1 -1)))
  (bind _____3 (Utilities|Add(IntVector2d) CurrentCorner (Utilities|Struct|MakeF_IntVector2d 0 1)))
  (bind _____4 (Utilities|Add(IntVector2d) CurrentCorner (Utilities|Struct|MakeF_IntVector2d 0 -1)))
  (bind _____5 (Utilities|Add(IntVector2d) CurrentCorner (Utilities|Struct|MakeF_IntVector2d 1 -1)))
  (bind _____6 (Utilities|Add(IntVector2d) CurrentCorner (Utilities|Struct|MakeF_IntVector2d 1 1)))
  (bind _____7 (Utilities|Add(IntVector2d) CurrentCorner (Utilities|Struct|MakeF_IntVector2d 1 0)))
  (bind _array (Utilities|Array|MakeArray 1 0 -1))
  (bind _array_2 (Utilities|Array|MakeArray 0 1 2))
  (bind _array_3 (Utilities|Array|MakeArray 0 -1 -2))
  (bind _array_4 (Utilities|Array|MakeArray 0 1 2))
  (bind _array_5 (Utilities|Array|MakeArray 0 -1 -2))
  (bind _array_6 (Utilities|Array|MakeArray 0 1 2))
  (bind _array_7 (Utilities|Array|MakeArray 0 -1 -2))
  (bind _array_8 (Utilities|Array|MakeArray 0 1 2))
  (bind _array_9 (Utilities|Array|MakeArray 0 -1 -2))
  (bind _cornermap (Variables|Default|GetCornerMap))
  (bind (_value _returnvalue) (Utilities|Map|Find _cornermap _____7))
  (bind (_value_2 _returnvalue_2) (Utilities|Map|Find _cornermap _____5))
  (bind (_value_3 _returnvalue_3) (Utilities|Map|Find :TargetMap _cornermap))
  (bind (_value_4 _returnvalue_4) (Utilities|Map|Find _cornermap ____))
  (bind (_value_5 _returnvalue_5) (Utilities|Map|Find _cornermap _____2))
  (bind (_value_6 _returnvalue_6) (Utilities|Map|Find _cornermap _____4))
  (bind (_value_7 _returnvalue_7) (Utilities|Map|Find _cornermap _____3))
  (bind (_value_8 _returnvalue_8) (Utilities|Map|Find _cornermap _____6))
  (bind _returnvalue_9 (- TestHeight _value_2))
  (bind _returnvalue_10 (- TestHeight _value_8))
  (bind _returnvalue_11 (- TestHeight _value))
  (bind _returnvalue_12 (- TestHeight _value_4))
  (bind _returnvalue_13 (- TestHeight _value_3))
  (bind _returnvalue_14 (- TestHeight _value_5))
  (bind _returnvalue_15 (- TestHeight _value_7))
  (bind _returnvalue_16 (- TestHeight _value_6))
  (LocalVariables|SetErrors 0)
  (if (== (Math|Integer|%(Integer) TestHeight 2) 0)
    ;[0.15 0.15 0.15 0.5 27] if test height is even (that is, on the border between tile spaces), add two errors for each of the neighboring tile spaces that our corner is part of where the heights are not all within the same tile
    ;;[0.15 0.15 0.15 0.5] if all of the northwest neighbors are not in the tile below or the tile above, add two errors
    (if (or (Math|Boolean|ANDBoolean (or (Utilities|Array|ContainsItem _array_6 _returnvalue_13) (not _returnvalue_3)) (or (Utilities|Array|ContainsItem _array_6 _returnvalue_12) (not _returnvalue_4)) (or (Utilities|Array|ContainsItem _array_6 _returnvalue_15) (not _returnvalue_7))) (Math|Boolean|ANDBoolean (or (Utilities|Array|ContainsItem _array_7 _returnvalue_13) (not _returnvalue_3)) (or (Utilities|Array|ContainsItem _array_7 _returnvalue_12) (not _returnvalue_4)) (or (Utilities|Array|ContainsItem _array_7 _returnvalue_15) (not _returnvalue_7))))
      _
      (else
        (LocalVariables|SetErrors (+ (LocalVariables|GetErrors) 2))))
    ;;[0.15 0.15 0.15 0.5] if all of the northeast neighbors are not in the tile below or the tile above, add two errors
    (if (or (Math|Boolean|ANDBoolean (or (Utilities|Array|ContainsItem _array_8 _returnvalue_15) (not _returnvalue_7)) (or (Utilities|Array|ContainsItem _array_8 _returnvalue_10) (not _returnvalue_8)) (or (Utilities|Array|ContainsItem _array_8 _returnvalue_11) (not _returnvalue))) (Math|Boolean|ANDBoolean (or (Utilities|Array|ContainsItem _array_9 _returnvalue_15) (not _returnvalue_7)) (or (Utilities|Array|ContainsItem _array_9 _returnvalue_10) (not _returnvalue_8)) (or (Utilities|Array|ContainsItem _array_9 _returnvalue_11) (not _returnvalue))))
      _
      (else
        (LocalVariables|SetErrors (+ (LocalVariables|GetErrors) 2))))
    ;;[0.15 0.15 0.15 0.5] if all of the southwest neighbors are not in the tile below or the tile above, add two errors
    (if (or (Math|Boolean|ANDBoolean (or (Utilities|Array|ContainsItem _array_4 _returnvalue_16) (not _returnvalue_6)) (or (Utilities|Array|ContainsItem _array_4 _returnvalue_14) (not _returnvalue_5)) (or (Utilities|Array|ContainsItem _array_4 _returnvalue_13) (not _returnvalue_3))) (Math|Boolean|ANDBoolean (or (Utilities|Array|ContainsItem _array_5 _returnvalue_16) (not _returnvalue_6)) (or (Utilities|Array|ContainsItem _array_5 _returnvalue_14) (not _returnvalue_5)) (or (Utilities|Array|ContainsItem _array_5 _returnvalue_13) (not _returnvalue_3))))
      _
      (else
        (LocalVariables|SetErrors (+ (LocalVariables|GetErrors) 2))))
    ;;[0.15 0.15 0.15 0.5] if all of the southeast neighbors are not in the tile below or the tile above, add two errors
    (if (or (Math|Boolean|ANDBoolean (or (Utilities|Array|ContainsItem _array_2 _returnvalue_11) (not _returnvalue)) (or (Utilities|Array|ContainsItem _array_2 _returnvalue_9) (not _returnvalue_2)) (or (Utilities|Array|ContainsItem _array_2 _returnvalue_16) (not _returnvalue_6))) (Math|Boolean|ANDBoolean (or (Utilities|Array|ContainsItem _array_3 _returnvalue_11) (not _returnvalue)) (or (Utilities|Array|ContainsItem _array_3 _returnvalue_9) (not _returnvalue_2)) (or (Utilities|Array|ContainsItem _array_3 _returnvalue_16) (not _returnvalue_6))))
      _
      (else
        (LocalVariables|SetErrors (+ (LocalVariables|GetErrors) 2))))
    (else
      ;[0.15 0.15 0.15 0.5 24] for each neighbor found to be not within 1 height, tally an error
      (Utilities|IncrementifTrue (LocalVariables|GetErrors) (Math|Boolean|NORBoolean (Utilities|Array|ContainsItem _array _returnvalue_12) (not _returnvalue_4)))
      (Utilities|IncrementifTrue (LocalVariables|GetErrors) (Math|Boolean|NORBoolean (Utilities|Array|ContainsItem _array _returnvalue_15) (not _returnvalue_7)))
      (Utilities|IncrementifTrue (LocalVariables|GetErrors) (Math|Boolean|NORBoolean (Utilities|Array|ContainsItem _array _returnvalue_10) (not _returnvalue_8)))
      (Utilities|IncrementifTrue (LocalVariables|GetErrors) (Math|Boolean|NORBoolean (Utilities|Array|ContainsItem _array _returnvalue_11) (not _returnvalue)))
      (Utilities|IncrementifTrue (LocalVariables|GetErrors) (Math|Boolean|NORBoolean (Utilities|Array|ContainsItem _array _returnvalue_9) (not _returnvalue_2)))
      (Utilities|IncrementifTrue (LocalVariables|GetErrors) (Math|Boolean|NORBoolean (Utilities|Array|ContainsItem _array _returnvalue_16) (not _returnvalue_6)))
      (Utilities|IncrementifTrue (LocalVariables|GetErrors) (Math|Boolean|NORBoolean (Utilities|Array|ContainsItem _array _returnvalue_14) (not _returnvalue_5)))
      (Utilities|IncrementifTrue (LocalVariables|GetErrors) (Math|Boolean|NORBoolean (Utilities|Array|ContainsItem _array _returnvalue_13) (not _returnvalue_3)))))
  (return (+ (Utilities|Int% (LocalVariables|GetErrors) 2) (/ (LocalVariables|GetErrors) 2))))