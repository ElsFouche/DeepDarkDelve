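; Generative grammar data asset that procedurally builds text, with accompanying name and tag lists, from a start phrase.
; Initialize loads rules from a data table, merging identical find phrases into weighted replacement lists.
; RunGeneration recursively rewrites the phrase, shuffling rules each pass and picking replacements by weighted roll, until none match.
; AtomicCollapse then swaps each symbol for a random word from its DT_AtomicLookup table, keeping unlisted symbols as literal text.
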(event `Initialize`
  (set `self.InitializationComplete` false)
  (`KismetArrayLibrary.Array_Clear` (`self.Rules`))
  (`self.RetrieveRules`))

(event `PrintRules`
  (`KismetSystemLibrary.PrintString` null "\n---------------------")
  (bind (_arrayelement _arrayindex) (`/Game/Blueprints/Libraries/BPML_Utilities.ForEachLoop_Real` (`self.Rules`) :!label _label)
    (:`LoopBody`
      (set `self.TempString` (`KismetStringLibrary.Concat_StrStr` "Rule #" (`KismetStringLibrary.Conv_IntToString` _arrayindex) "\nReplace " (`self.toString` (break `/Game/Data/Procedural/Grammar/F_GGRule` _arrayelement)) " with: " (`self.toString` (`|GetArrayItem` (break `/Game/Data/Procedural/Grammar/F_ReplacementList` (`.Replacements_6_104C94E527BF4B7BA4EFEC3377B9582D` (break `/Game/Data/Procedural/Grammar/F_GGRule` _arrayelement)))))))
      (bind (_arrayelement_2 _arrayindex_2) (`/Game/Blueprints/Libraries/BPML_Utilities.ForEachLoop_Real` (break `/Game/Data/Procedural/Grammar/F_ReplacementList` (`.Replacements_6_104C94E527BF4B7BA4EFEC3377B9582D` (break `/Game/Data/Procedural/Grammar/F_GGRule` _arrayelement))) :!label _label_2)
        (:`LoopBody`
          (if (== _arrayindex_2 0)
            (goto _label_2 :!via `Continue`)
            (else
              (set `self.TempString` (`KismetStringLibrary.Concat_StrStr` (`self.TempString`) "\nOR " (`self.toString` _arrayelement_2)))
              (goto _label_2 :!via `Continue`))))
        (:`Completed`
          (`KismetSystemLibrary.PrintString` null (`KismetStringLibrary.Concat_StrStr` (`self.TempString`) "\n---------------------\n"))
          (goto _label :!via `Continue`))))))

(event `RetrieveRules`
  (bind _rulelookuptable (`self.RuleLookupTable`))
  ;[0.15 0.15 0.15 0.5 36] Retrieve rules from data table
  (if (== (`DataTableFunctionLibrary.GetDataTableRowStruct` _rulelookuptable) "/Game/Data/Procedural/Grammar/F_RowRule.F_RowRule")
    (bind _outrownames (`DataTableFunctionLibrary.GetDataTableRowNames` _rulelookuptable))
    (bind _arrayelement (`/Game/Blueprints/Libraries/BPML_Utilities.ForEachLoop_Real` _outrownames :!label _label_3)
      (:`LoopBody`
        (bind _returnvalue (`|GetDataTableRow` _rulelookuptable _arrayelement)
          (:`then`
            (bind (_arrayelement_2 _arrayindex) (`/Game/Blueprints/Libraries/BPML_Utilities.ForEachLoop_Real` (`self.Rules`) :!label _label_4)
              (:`LoopBody`
                (bind (_find _replacements) (break `/Game/Data/Procedural/Grammar/F_GGRule` _arrayelement_2))
                (bind (_find_2 _replace _weight) (break `/Game/Data/Procedural/Grammar/F_RowRule` _returnvalue))
                (if (`KismetArrayLibrary.Array_Identical` (break `/Game/Data/Procedural/Grammar/F_Phrase` _find) _find_2)
                  (bind (_replacements_2 _weights) (break `/Game/Data/Procedural/Grammar/F_ReplacementList` _replacements))
                  (bind _output_get (set `self.TempReplacements` _replacements_2))
                  (`KismetArrayLibrary.Array_Add` _output_get (make `/Game/Data/Procedural/Grammar/F_Phrase` _replace))
                  (bind _output_get_2 (set `self.TempWeights` _weights))
                  (`KismetArrayLibrary.Array_Add` _output_get_2 _weight)
                  (`KismetArrayLibrary.Array_Set` (`self.Rules`) _arrayindex (make `/Game/Data/Procedural/Grammar/F_GGRule` (make `/Game/Data/Procedural/Grammar/F_Phrase` (break `/Game/Data/Procedural/Grammar/F_Phrase` _find)) (make `/Game/Data/Procedural/Grammar/F_ReplacementList` (`self.TempReplacements`) (`self.TempWeights`))))
                  (goto _label_3 :!via `Continue`)
                  (else
                    (goto _label_4 :!via `Continue`))))
              (:`Completed`
                (`KismetArrayLibrary.Array_Add` (`self.Rules`) (make `/Game/Data/Procedural/Grammar/F_GGRule` (make `/Game/Data/Procedural/Grammar/F_Phrase` _find_2) (make `/Game/Data/Procedural/Grammar/F_ReplacementList` (`|MakeArray` (make `/Game/Data/Procedural/Grammar/F_Phrase` _replace) :!type "/Game/Data/Procedural/Grammar/F_Phrase Structure") (`|MakeArray` _weight))))
                (goto _label_3 :!via `Continue`))))))
      (:`Completed`
        (set `self.InitializationComplete` true)))
    (else
      (`KismetSystemLibrary.PrintString` null (`KismetStringLibrary.Concat_StrStr` "Improper data table implementation!\n- Rule lookup table in \"" (`KismetSystemLibrary.GetObjectName` self) "\" is invalid.\n- All generative grammar rule tables must use the `F_RowRule` structure") true true (struct :`G` 0.66 :`B` 1.0 :`A` 1.0) 5.0))))

(event `RunGeneration`
  (bind _array (`|MakeArray`))
  (set `self.CurrentPhrase` (`self.StartPhrase`))
  (set `self.GenerationComplete` false)
  (set `self.OutputString` "")
  (set `self.OutputTags` _array)
  (set `self.OutputNames` _array)
  (`self.FindAndReplace`))

(event `FindAndReplace`
  (bind _currentphrase_names (break `/Game/Data/Procedural/Grammar/F_Phrase` (`self.CurrentPhrase`)))
  (bind _currentphrase_names_2 (break `/Game/Data/Procedural/Grammar/F_Phrase` (`self.CurrentPhrase`)))
  (bind _currentrule (`self.CurrentRule`))
  (bind _startindex (`self.StartIndex`))
  (bind _currentphrase_names_3 (break `/Game/Data/Procedural/Grammar/F_Phrase` (`self.CurrentPhrase`)))
  (bind _currentrule_2 (`self.CurrentRule`))
  (bind _currentphrasebeginning_names (break `/Game/Data/Procedural/Grammar/F_Phrase` (`self.CurrentPhraseBeginning`)))
  (bind _currentphraseending_names (break `/Game/Data/Procedural/Grammar/F_Phrase` (`self.CurrentPhraseEnding`)))
  (bind _currentphrase_names_4 (break `/Game/Data/Procedural/Grammar/F_Phrase` (`self.CurrentPhrase`)))
  (bind _rules (`self.Rules`))
  ;[0.15 0.15 0.15 0.5 36] Attempt to find and replace based on the grammar rules
  (`KismetArrayLibrary.Array_Shuffle` _rules)
  (bind (_arrayelement _arrayindex) (`/Game/Blueprints/Libraries/BPML_Utilities.ForEachLoop_Real` _rules :!label _label_5)
    (:`LoopBody`
      (set `self.CurrentRule` _arrayelement)
      ;; try to find a match with the current rule
      (bind (_arrayelement_2 _arrayindex_2) (`/Game/Blueprints/Libraries/BPML_Utilities.ForEachLoop_Real` _currentphrase_names_4 :!label _label_6)
        (:`LoopBody`
          (if (== _arrayelement_2 (`|GetArrayItem` (break `/Game/Data/Procedural/Grammar/F_Phrase` (break `/Game/Data/Procedural/Grammar/F_GGRule` _currentrule))))
            (set `self.StartIndex` _arrayindex_2)
            (bind _index (`/Game/Blueprints/Libraries/BPML_Utilities.ForLoop_Real` 1 (`KismetArrayLibrary.Array_LastIndex` (break `/Game/Data/Procedural/Grammar/F_Phrase` (break `/Game/Data/Procedural/Grammar/F_GGRule` _currentrule))) :!label _label_7)
              (:`LoopBody`
                (bind _returnvalue (+ _index _arrayindex_2))
                (if (`KismetArrayLibrary.Array_IsValidIndex` _currentphrase_names _returnvalue)
                  (if (== (`|GetArrayItem` _currentphrase_names _returnvalue) (`|GetArrayItem` (break `/Game/Data/Procedural/Grammar/F_Phrase` (break `/Game/Data/Procedural/Grammar/F_GGRule` _currentrule)) _arrayindex_2))
                    (goto _label_7 :!via `Continue`)
                    (else
                      (goto _label_6 :!via `Continue`)))
                  (else
                    (goto _label_6 :!via `Continue`))))
              (:`Complete`
                ;; Rule Applies! chop the current phrase into a beginning and end bit
                (bind _subarray (`/Game/Blueprints/Libraries/BPML_Utilities.Subarray` _currentphrase_names_3 0 (- _startindex 1))
                  (:`__`
                    (set `self.CurrentPhraseBeginning` (make `/Game/Data/Procedural/Grammar/F_Phrase` _subarray))
                    (bind _subarray_2 (`/Game/Blueprints/Libraries/BPML_Utilities.Subarray` _currentphrase_names_2 (+ _startindex (`KismetArrayLibrary.Array_Length` (break `/Game/Data/Procedural/Grammar/F_Phrase` (break `/Game/Data/Procedural/Grammar/F_GGRule` (`self.CurrentRule`))))) (`KismetArrayLibrary.Array_LastIndex` _currentphrase_names_3))
                      (:`__`
                        (set `self.CurrentPhraseEnding` (make `/Game/Data/Procedural/Grammar/F_Phrase` _subarray_2))
                        ;; pick a replacement from the possiblities provided by the current rule
                        (set `self.Roll` (`KismetMathLibrary.RandomFloatInRange` 0.0 (`self.SumOfFloats` (`.Weights_12_F3CCABA5B241453F83BDC4AA707727AD` (break `/Game/Data/Procedural/Grammar/F_ReplacementList` (`.Replacements_6_104C94E527BF4B7BA4EFEC3377B9582D` (break `/Game/Data/Procedural/Grammar/F_GGRule` (`self.CurrentRule`))))))))
                        (bind (_arrayelement_3 _arrayindex_3) (`/Game/Blueprints/Libraries/BPML_Utilities.ForEachLoop_Real` (`.Weights_12_F3CCABA5B241453F83BDC4AA707727AD` (break `/Game/Data/Procedural/Grammar/F_ReplacementList` (`.Replacements_6_104C94E527BF4B7BA4EFEC3377B9582D` (break `/Game/Data/Procedural/Grammar/F_GGRule` _currentrule_2)))) :!label _label_8)
                          (:`LoopBody`
                            (bind _output_get (set `self.Roll` (- (`self.Roll`) _arrayelement_3)))
                            (if (> _output_get 0.0)
                              (goto _label_8 :!via `Continue`)
                              (else
                                ;; construct next phrase to operate on, using the beginning and end fragments, and the chosen replacement from the rule
                                (set `self.tempPhrase` _currentphrasebeginning_names)
                                (bind _output_names (break `/Game/Data/Procedural/Grammar/F_Phrase` (`|GetArrayItem` (break `/Game/Data/Procedural/Grammar/F_ReplacementList` (`.Replacements_6_104C94E527BF4B7BA4EFEC3377B9582D` (break `/Game/Data/Procedural/Grammar/F_GGRule` _currentrule_2))) _arrayindex_3)))
                                (bind _arrayelement_4 (`/Game/Blueprints/Libraries/BPML_Utilities.ForEachLoop_Real` _output_names :!label _label_9)
                                  (:`LoopBody`
                                    (`KismetArrayLibrary.Array_Add` (`self.tempPhrase`) _arrayelement_4)
                                    (goto _label_9 :!via `Continue`))
                                  (:`Completed`
                                    (bind _arrayelement_5 (`/Game/Blueprints/Libraries/BPML_Utilities.ForEachLoop_Real` _currentphraseending_names :!label _label_10)
                                      (:`LoopBody`
                                        (`KismetArrayLibrary.Array_Add` (`self.tempPhrase`) _arrayelement_5)
                                        (goto _label_10 :!via `Continue`))
                                      (:`Completed`
                                        (set `self.CurrentPhrase` (make `/Game/Data/Procedural/Grammar/F_Phrase` (`self.tempPhrase`)))
                                        ;; if it made it this far, a replacement was made, so try again
                                        (`self.FindAndReplace`)))))))))))))))
            (else
              (goto _label_6 :!via `Continue`))))
        (:`Completed`
          (goto _label_5 :!via `Continue`))))
    (:`Completed`
      (`self.AtomicCollapse`))))

(event `AtomicCollapse`
  (bind (_tempworddata_word _tempworddata_tags) (break `/Game/Data/Procedural/Grammar/F_RowAtomic` (`self.TempWordData`)))
  (bind _currentphrase_names (break `/Game/Data/Procedural/Grammar/F_Phrase` (`self.CurrentPhrase`)))
  ; if no replacements were made on the last run of find and replace, it is time to collapse the atomics
  (set `self.OutputString` "")
  (bind _arrayelement (`/Game/Blueprints/Libraries/BPML_Utilities.ForEachLoop_Real` _currentphrase_names :!label _label_11)
    (:`LoopBody`
      (bind _returnvalue (`|GetDataTableRow` "/Game/Data/Procedural/Grammar/DT_AtomicLookup.DT_AtomicLookup" _arrayelement)
        (:`then`
          (if (== (`DataTableFunctionLibrary.GetDataTableRowStruct` (break `/Game/Data/Procedural/Grammar/F_RowDTLookup` _returnvalue)) "/Game/Data/Procedural/Grammar/F_RowAtomic.F_RowAtomic")
            (bind _outrownames (`DataTableFunctionLibrary.GetDataTableRowNames` (break `/Game/Data/Procedural/Grammar/F_RowDTLookup` _returnvalue)))
            (bind _returnvalue_2 (`|GetDataTableRow` (break `/Game/Data/Procedural/Grammar/F_RowDTLookup` _returnvalue) (`KismetArrayLibrary.Array_Random` _outrownames))
              (:`then`
                (set `self.TempWordData` _returnvalue_2)
                (set `self.OutputString` (`KismetStringLibrary.Concat_StrStr` (`self.OutputString`) " " _tempworddata_word) :!label _label_12)
                (`KismetArrayLibrary.Array_Add` (`self.OutputNames`) (`KismetStringLibrary.Conv_StringToName` _tempworddata_word))
                (bind _arrayelement_2 (`/Game/Blueprints/Libraries/BPML_Utilities.ForEachLoop_Real` _tempworddata_tags :!label _label_13)
                  (:`LoopBody`
                    (`KismetArrayLibrary.Array_AddUnique` (`self.OutputTags`) _arrayelement_2)
                    (goto _label_13 :!via `Continue`))
                  (:`Completed`
                    (goto _label_11 :!via `Continue`)))))
            (else
              (`KismetSystemLibrary.PrintString` null (`KismetStringLibrary.Concat_StrStr` "Improper data table implementation!\n- Atomic data table for \"" (`KismetStringLibrary.Conv_NameToString` _arrayelement) "\" uses the wrong struct or was not found.\nAll atomic data tables must use the `F_RowAtomic` structure")))))
        (:`RowNotFound`
          (set `self.TempWordData` (make `/Game/Data/Procedural/Grammar/F_RowAtomic` (`KismetStringLibrary.Conv_NameToString` _arrayelement)))
          (goto _label_12))))
    (:`Completed`
      (set `self.GenerationComplete` true))))

(fn `GetOutputNames`
  (returns (OutputNames :type "Array of Name"))
  (if (`self.GenerationComplete`)
    (return (`self.OutputNames`))
    (else
      (return (`|MakeArray`)))))

(fn `GetOutputString`
  (returns (OutputString :type String))
  (if (`self.GenerationComplete`)
    (return (`self.OutputString`))
    (else
      (return ""))))

(fn `GetOutputTags`
  (returns (OutputTags :type "Array of Name"))
  (if (`self.GenerationComplete`)
    (return (`self.OutputTags`))
    (else
      (return (`|MakeArray`)))))

(fn `isGenerationComplete`
  (returns (_ :type Boolean))
  (return (`self.GenerationComplete`)))

(fn `SumOfFloats`
  (params (_ :type "Array of Float (double-precision)"))
  (returns (__ :type "Float (double-precision)"))
  (locals (acc :type "Float (double-precision)"))
  (for _array_element _
    (bind _output_get (set `local.acc` (+ (`local.acc`) _array_element))))
  (return _output_get))

(fn `toString`
  (params (__ :type "/Game/Data/Procedural/Grammar/F_Phrase Structure"))
  (returns (___ :type String))
  (locals (LocalString :type String))
  (set `local.LocalString` "")
  (bind _arrayelement (`/Game/Blueprints/Libraries/BPML_Utilities.ForEachLoop_Real` ___Names_3_3E8FE8D7469448C9B89B3493BF30D906 :!label _label)
    (:`LoopBody`
      (set `local.LocalString` (`KismetStringLibrary.Concat_StrStr` (`local.LocalString`) " " (`KismetStringLibrary.Conv_NameToString` _arrayelement)))
      (goto _label :!via `Continue`))
    (:`Completed`
      (return (`local.LocalString`)))))