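; Blueprint function library of general math and array helpers.
; TimeConversion solves for whichever of distance, rate or time is missing, optionally measuring distance between two points, and returns -1s unless exactly one is unknown.
; Other helpers cover vector angles, ping-pong indices, rounding to multiples via a sign-adjusted modulo, powers of two, array sums and vector pop/shift.
; FloatPrecision truncates decimals by splitting the number as a string rather than rounding.
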(fn `%`
  (params (_ :type "Float (double-precision)") (__ :type "Float (double-precision)"))
  (returns (___ :type "Float (double-precision)"))
  (bind _returnvalue (mod _ __))
  (return (`KismetMathLibrary.SelectFloat` _returnvalue (+ _returnvalue __) (>= _ 0.0))))

(fn `AngleBetweenTwoVectors`
  (params (V1 :type "Vector Structure") (V2 :type "Vector Structure"))
  (returns (AngleDegrees :type "Float (double-precision)"))
  (return (`KismetMathLibrary.DegAcos` (`KismetMathLibrary.Dot_VectorVector` (`KismetMathLibrary.Normal` V1 0.001) (`KismetMathLibrary.Normal` V2 0.001)))))

(fn `FloatPrecision`
  (params (InFloat :type "Float (double-precision)") (DecimalPrecision :type Integer :default 2))
  (returns (OutFloat :type "Float (double-precision)") (OutString :type String))
  (bind _returnvalue (`KismetStringLibrary.ParseIntoArray` (`KismetStringLibrary.Conv_DoubleToString` InFloat) "."))
  (bind _returnvalue_2 (`KismetStringLibrary.Concat_StrStr` (`|GetArrayItem` _returnvalue) "." (`KismetStringLibrary.GetSubstring` (`|GetArrayItem` _returnvalue 1) 0 DecimalPrecision)))
  (return (`KismetStringLibrary.Conv_StringToDouble` _returnvalue_2) _returnvalue_2))

(fn `PingPong`
  (params (InIndex :type Integer) (Period :type Integer))
  (returns (OutIndex :type Integer))
  (bind _returnvalue (* Period 2))
  (bind _returnvalue_2 (mod InIndex _returnvalue))
  (return (`KismetMathLibrary.SelectInt` _returnvalue_2 (- _returnvalue _returnvalue_2) (< _returnvalue_2 Period))))

(fn `Pop(Vector)`
  (params (_ :type "Array of Vector Structure"))
  (returns (__ :type "Vector Structure"))
  (locals (TempVector :type "Vector Structure"))
  (bind _returnvalue (`KismetArrayLibrary.Array_LastIndex` _))
  (bind _output_get (set `local.TempVector` (`|GetArrayItem` _ _returnvalue)))
  (`KismetArrayLibrary.Array_Remove` _ _returnvalue)
  (return _output_get))

(fn `PowerOfTwo`
  (params (_ :type Integer))
  (returns (__ :type Integer))
  (locals (acc :type Integer))
  (set `local.acc` 1)
  (`/Game/Blueprints/Libraries/BPML_Utilities.ForLoop_Real` 1 _ :!label _label
    (:`LoopBody`
      (set `local.acc` (* 2 (`local.acc`)))
      (goto _label :!via `Continue`))
    (:`Complete`
      (return (`local.acc`)))))

(fn `RoundAround`
  (params (ValueToRound :type "Float (double-precision)") (RoundBy :type Integer))
  (returns (RoundedValue :type Integer))
  (bind _returnvalue (`KismetMathLibrary.Conv_IntToDouble` RoundBy))
  (bind _returnvalue_2 (* (`KismetMathLibrary.FTrunc` (`KismetMathLibrary.SafeDivide` ValueToRound _returnvalue)) RoundBy))
  (return (`KismetMathLibrary.SelectInt` _returnvalue_2 (+ _returnvalue_2 RoundBy) (< (`/Game/Blueprints/Libraries/BPML_Math.%` ValueToRound _returnvalue) (/ RoundBy 2)))))

(fn `Shift(Vector)`
  (params (_ :type "Array of Vector Structure"))
  (returns (__ :type "Vector Structure"))
  (locals (TempVector :type "Vector Structure"))
  (bind _output_get (set `local.TempVector` (`|GetArrayItem` _)))
  (`KismetArrayLibrary.Array_Remove` _)
  (return _output_get))

(fn `SumOfFloats`
  (params (_ :type "Array of Float (double-precision)"))
  (returns (__ :type "Float (double-precision)"))
  (locals (acc :type "Float (double-precision)"))
  (for _array_element _
    (bind _output_get (set `local.acc` (+ (`local.acc`) _array_element))))
  (return _output_get))

(fn `SumOfInts`
  (params (_ :type "Array of Integer"))
  (returns (__ :type Integer))
  (locals (acc :type Integer))
  (for _array_element _
    (bind _output_get (set `local.acc` (+ (`local.acc`) _array_element))))
  (return _output_get))

(fn `TimeConversion`
  (params (Distance :type "Float (double-precision)") (Start :type "Vector Structure") (End :type "Vector Structure") (Rate :type "Float (double-precision)") (Time :type "Float (double-precision)"))
  (returns (OutDistance :type "Float (double-precision)") (OutRate :type "Float (double-precision)") (OutTime :type "Float (double-precision)"))
  (locals (LocalRate :type "Float (double-precision)" :default -1.0) (LocalTime :type "Float (double-precision)" :default -1.0) (LocalDistance :type "Float (double-precision)" :default -1.0) (SolveFor :type "Array of Integer"))
  (bind _returnvalue (`KismetMathLibrary.Vector_Distance` Start End))
  (bind _solvefor (`local.SolveFor`))
  (if (> Distance 0.0)
    (set `local.LocalDistance` Distance)
    (elif (> _returnvalue 0.0)
      (set `local.LocalDistance` _returnvalue)
      (else
        (`KismetArrayLibrary.Array_Add` (`local.SolveFor`) 1))))
  (if (> Rate 0.0)
    (set `local.LocalRate` Rate)
    (else
      (`KismetArrayLibrary.Array_Add` (`local.SolveFor`) 2)))
  (if (> Time 0.0)
    (set `local.LocalTime` Time)
    (else
      (`KismetArrayLibrary.Array_Add` (`local.SolveFor`) 3)))
  (if (and (== (`KismetArrayLibrary.Array_Length` _solvefor) 1) (`KismetArrayLibrary.Array_IsValidIndex` _solvefor))
    (switch `int` (`|GetArrayItem` _solvefor)
      (:`Default`
        _)
      (:`0`
        _)
      (:`1`
        (`KismetArrayLibrary.Array_Clear` (`local.SolveFor`))
        (return (* (`local.LocalTime`) (`local.LocalRate`)) (`local.LocalRate`) (`local.LocalTime`)))
      (:`2`
        (`KismetArrayLibrary.Array_Clear` (`local.SolveFor`))
        (return (`local.LocalDistance`) (`KismetMathLibrary.SafeDivide` (`local.LocalDistance`) (`local.LocalTime`)) (`local.LocalTime`)))
      (:`3`
        (`KismetArrayLibrary.Array_Clear` (`local.SolveFor`))
        (return (`local.LocalDistance`) (`local.LocalRate`) (`KismetMathLibrary.SafeDivide` (`local.LocalDistance`) (`local.LocalRate`))))))
  (`KismetArrayLibrary.Array_Clear` (`local.SolveFor`))
  (return -1.0 -1.0 -1.0))