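; Blueprint function library that converts between world positions and integer tile coordinates on the game's grid.
; The cell size comes from the default GridSize, with any zero axis replaced by 1 to avoid division by zero.
; World-to-tile functions divide by that size, rounding X and Y to the nearest tile but truncating Z.
; ToWorldPosition reverses this by multiplying tile coordinates by the cell size.
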(fn `GetDefaultGridSize`
  (returns (GridSize :type "IntVector Structure"))
  (locals (Defaults :type "/Game/Data/Global/PDA_GlobalData Object Reference" :default "/Game/Data/Global/PDA_GlobalData.PDA_GlobalData_C'/Game/Data/Global/DA_GlobalDefaults.DA_GlobalDefaults'"))
  (bind (_gridsize_x _gridsize_y _gridsize_z) (break `IntVector` (`/Game/Data/Global/PDA_GlobalData.GridSize` (`local.Defaults`))))
  (return (make `IntVector` (`KismetMathLibrary.SelectInt` 1 _gridsize_x (== _gridsize_x 0)) (`KismetMathLibrary.SelectInt` 1 _gridsize_y (== _gridsize_y 0)) (`KismetMathLibrary.SelectInt` 1 _gridsize_z (== _gridsize_z 0)))))

(fn `IntVectToTile`
  (params (Location :type "IntVector Structure"))
  (returns (GridCorrected :type "IntVector Structure"))
  (bind (_returnvalue_x _returnvalue_y _returnvalue_z) (`KismetMathLibrary.BreakVector` (/ (`KismetMathLibrary.Conv_IntVectorToVector` Location) (`self.GetDefaultGridSize` null))))
  (return (make `IntVector` (`KismetMathLibrary.Round` _returnvalue_x) (`KismetMathLibrary.Round` _returnvalue_y) (`KismetMathLibrary.FTrunc` _returnvalue_z))))

(fn `ToTilePosition`
  (params (_ :type "Vector Structure") (__WorldContext :type "Object Object Reference"))
  (returns (__ :type "IntVector Structure"))
  (bind (_returnvalue_x _returnvalue_y _returnvalue_z) (`KismetMathLibrary.BreakVector` (/ _ (`self.GetDefaultGridSize` null))))
  (return (make `IntVector` (`KismetMathLibrary.Round` _returnvalue_x) (`KismetMathLibrary.Round` _returnvalue_y) (`KismetMathLibrary.FTrunc` _returnvalue_z))))

(fn `ToWorldPosition`
  (params (_ :type "IntVector Structure") (__WorldContext :type "Object Object Reference"))
  (returns (__ :type "Vector Structure"))
  (return (`KismetMathLibrary.Conv_IntVectorToVector` (`/Game/Blueprints/Libraries/BPML_VectorMath.Multiply (IntVector)` _ (`self.GetDefaultGridSize` null)))))

(fn `VectToTile`
  (params (Location :type "Vector Structure"))
  (returns (GridCorrected :type "IntVector Structure"))
  (bind (_returnvalue_x _returnvalue_y _returnvalue_z) (`KismetMathLibrary.BreakVector` (/ Location (`self.GetDefaultGridSize` null))))
  (return (make `IntVector` (`KismetMathLibrary.Round` _returnvalue_x) (`KismetMathLibrary.Round` _returnvalue_y) (`KismetMathLibrary.FTrunc` _returnvalue_z))))