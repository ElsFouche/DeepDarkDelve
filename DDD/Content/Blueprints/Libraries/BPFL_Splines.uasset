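; Blueprint function library that builds jump-arc splines and runs collision traces along splines.
; FindJumpSpline reshapes a given spline into a two-point arc, deriving tangents from a right-isosceles triangle in the vertical plane, clamped in angle and scaled by Steepness.
; The trace functions line-trace between tolerance-based polyline points.
; Variants return the first hit, one result per segment including misses, or all multi-trace hits per segment.
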(fn `FindJumpSpline`
  (params (StartLocation :type "Vector Structure") (EndLocation :type "Vector Structure") (Steepness :type "Float (double-precision)" :default 0.65) (InSpline :type "SplineComponent Object Reference (by ref)"))
  (returns (JumpSpline :type "SplineComponent Object Reference") (Success :type Boolean))
  (locals (Spline :type "SplineComponent Object Reference") (Start :type "Vector Structure") (End :type "Vector Structure") (Normal :type "Vector Structure") (ScalingFactor :type "Float (double-precision)" :default 0.65))
  (bind _returnvalue (`KismetMathLibrary.Vector_Up`))
  (bind _returnvalue_2 (`KismetMathLibrary.Vector_Up`))
  (bind _spline (`local.Spline`))
  (bind _scalingfactor (`local.ScalingFactor`))
  (bind _normal (`local.Normal`))
  (bind _returnvalue_3 (/ (- (`local.End`) (`local.Start`)) 2.0))
  (bind _returnvalue_4 (+ _returnvalue_3 (`local.Start`) (`KismetMathLibrary.RotateAngleAxis` _returnvalue_3 90.0 (`local.Normal`))))
  (bind _returnvalue_5 (- _returnvalue_4 (`local.End`)))
  (bind _returnvalue_6 (- _returnvalue_4 (`local.Start`)))
  (bind _angledegrees (`/Game/Blueprints/Libraries/BPFL_Utilities.AngleBetweenTwoVectors` _returnvalue_5 _returnvalue))
  (bind _angledegrees_2 (`/Game/Blueprints/Libraries/BPFL_Utilities.AngleBetweenTwoVectors` _returnvalue_6 _returnvalue_2))
  (bind _returnvalue_7 (`KismetMathLibrary.SelectFloat` (* _angledegrees -1.0) _angledegrees (`KismetMathLibrary.NearlyEqual_FloatFloat` (+ _angledegrees (`/Game/Blueprints/Libraries/BPFL_Utilities.AngleBetweenTwoVectors` _returnvalue (- (`local.Start`) (`local.End`)))) 45.0 0.01)))
  (bind _returnvalue_8 (`KismetMathLibrary.SelectFloat` (* _angledegrees_2 -1.0) _angledegrees_2 (`KismetMathLibrary.NearlyEqual_FloatFloat` (+ _angledegrees_2 (`/Game/Blueprints/Libraries/BPFL_Utilities.AngleBetweenTwoVectors` _returnvalue_2 (- (`local.End`) (`local.Start`)))) 45.0 0.01)))
  (set `local.Spline` InSpline)
  (set `local.ScalingFactor` Steepness)
  (set `local.Start` StartLocation)
  (set `local.End` EndLocation)
  (set `local.Normal` (`KismetMathLibrary.Cross_VectorVector` (- (`local.End`) (`local.Start`)) (`KismetMathLibrary.Vector_Up`)))
  (`/Engine/EditorBlueprintResources/StandardMacros.IsValid` _spline
    (:`Is Valid`
      (`SplineComponent.ClearSplinePoints` _spline true)
      (`SplineComponent.AddSplinePointAtIndex` _spline (`local.Start`) 0 "World" true)
      (`SplineComponent.AddSplinePointAtIndex` _spline (`local.End`) 1 "World" true)
      (`SplineComponent.SetTangentsAtSplinePoint` _spline 0 (0.0 0.0 0.0) (* (`KismetMathLibrary.RotateAngleAxis` _returnvalue_6 (- (`KismetMathLibrary.ClampAngle` _returnvalue_8 0.0 70.0) _returnvalue_8) (`KismetMathLibrary.NegateVector` _normal)) _scalingfactor) "Local" true)
      (`SplineComponent.SetTangentsAtSplinePoint` _spline 1 (`KismetMathLibrary.NegateVector` (* _scalingfactor (`KismetMathLibrary.RotateAngleAxis` _returnvalue_5 (- (`KismetMathLibrary.ClampAngle` _returnvalue_7 0.0 70.0) _returnvalue_7) _normal))) (0.0 0.0 0.0) "Local" true)
      (return _spline true))
    (:`Is Not Valid`
      (`KismetSystemLibrary.PrintString` null "Invalid Spline")
      (return (`local.Spline`) false))))

(fn `SplineTraceByChannel`
  (params (SplineToTrace :type "SplineComponent Object Reference") (Tolerance :type "Float (double-precision)" :default 1.0) (TraceChannel :type "ETraceTypeQuery Enum" :default "TraceTypeQuery1") (TraceComplex :type Boolean) (ActorsToIgnore :type "Array of Actor Object Reference") (DrawDebugType :type "EDrawDebugTrace Enum" :default "ForDuration") (IgnoreSelf :type Boolean :default true) (TraceColor :type "LinearColor Structure" :default (struct :`R` 0.935425 :`G` 1.0 :`B` 0.239583 :`A` 1.0)) (TraceHitColor :type "LinearColor Structure" :default (struct :`G` 0.949118 :`B` 1.0 :`A` 1.0)) (DrawTime :type "Float (double-precision)" :default 5.0))
  (returns (Hit :type "HitResult Structure") (`isHit?` :type Boolean))
  (locals (LocalHit :type "HitResult Structure") (isHit :type Boolean))
  (bind _outpoints (`SplineComponent.ConvertSplineToPolyLine` SplineToTrace "World" (`KismetMathLibrary.SelectFloat` 1.0 Tolerance (`KismetMathLibrary.NearlyEqual_FloatFloat` Tolerance 0.0 0.009))))
  (for (_array_element _array_index) _outpoints
    (bind (_outhit _returnvalue) (`KismetSystemLibrary.LineTraceSingle` null _array_element (`KismetMathLibrary.SelectVector` (`|GetArrayItem` _outpoints (+ 1 _array_index)) _array_element (< _array_index (- (`KismetArrayLibrary.Array_Length` _outpoints) 1))) (`local.TraceChannel`) (`local.TraceComplex`) (`local.ActorsToIgnore`) (`local.DrawDebugType`) (`local.IgnoreSelf`) (`local.TraceColor`) (`local.TraceHitColor`) (`local.DrawTime`)))
    (if _returnvalue
      (set `local.LocalHit` _outhit)
      (bind _output_get (set `local.isHit` true))
      (break)))
  (return (`local.LocalHit`) _output_get))

(fn `SplineTraceByChannelMulti`
  (params (SplineToTrace :type "SplineComponent Object Reference") (Tolerance :type "Float (double-precision)" :default 1.0) (TraceChannel :type "ETraceTypeQuery Enum" :default "TraceTypeQuery1") (TraceComplex :type Boolean) (ActorsToIgnore :type "Array of Actor Object Reference") (DrawDebugType :type "EDrawDebugTrace Enum" :default "ForDuration") (IgnoreSelf :type Boolean :default true) (TraceColor :type "LinearColor Structure" :default (struct :`R` 0.935425 :`G` 1.0 :`B` 0.239583 :`A` 1.0)) (TraceHitColor :type "LinearColor Structure" :default (struct :`G` 0.949118 :`B` 1.0 :`A` 1.0)) (DrawTime :type "Float (double-precision)" :default 5.0))
  (returns (Hits :type "Array of HitResult Structure"))
  (locals (AllHits :type "Array of HitResult Structure"))
  (bind _outpoints (`SplineComponent.ConvertSplineToPolyLine` SplineToTrace "World" (`KismetMathLibrary.SelectFloat` 1.0 Tolerance (`KismetMathLibrary.NearlyEqual_FloatFloat` Tolerance 0.0 0.009))))
  (for (_array_element _array_index) _outpoints
    (bind _outhit (`KismetSystemLibrary.LineTraceSingle` null _array_element (`KismetMathLibrary.SelectVector` (`|GetArrayItem` _outpoints (+ 1 _array_index)) _array_element (< _array_index (- (`KismetArrayLibrary.Array_Length` _outpoints) 1))) (`local.TraceChannel`) (`local.TraceComplex`) (`local.ActorsToIgnore`) (`local.DrawDebugType`) (`local.IgnoreSelf`) (`local.TraceColor`) (`local.TraceHitColor`) (`local.DrawTime`)))
    (`KismetArrayLibrary.Array_Add` (`local.AllHits`) _outhit))
  (return (`local.AllHits`)))

(fn `SplineTraceByChannelMultiHighPrecision`
  (params (SplineToTrace :type "SplineComponent Object Reference") (Tolerance :type "Float (double-precision)" :default 1.0) (TraceChannel :type "ETraceTypeQuery Enum" :default "TraceTypeQuery1") (TraceComplex :type Boolean) (ActorsToIgnore :type "Array of Actor Object Reference") (DrawDebugType :type "EDrawDebugTrace Enum" :default "ForDuration") (IgnoreSelf :type Boolean :default true) (TraceColor :type "LinearColor Structure" :default (struct :`R` 0.935425 :`G` 1.0 :`B` 0.239583 :`A` 1.0)) (TraceHitColor :type "LinearColor Structure" :default (struct :`G` 0.949118 :`B` 1.0 :`A` 1.0)) (DrawTime :type "Float (double-precision)" :default 5.0))
  (returns (Hits :type "Array of HitResult Structure"))
  (locals (AllHits :type "Array of HitResult Structure"))
  (bind _outpoints (`SplineComponent.ConvertSplineToPolyLine` SplineToTrace "World" (`KismetMathLibrary.SelectFloat` 1.0 Tolerance (`KismetMathLibrary.NearlyEqual_FloatFloat` Tolerance 0.0 0.009))))
  (for (_array_element _array_index) _outpoints
    (bind _outhits (`KismetSystemLibrary.LineTraceMulti` null _array_element (`KismetMathLibrary.SelectVector` (`|GetArrayItem` _outpoints (+ 1 _array_index)) _array_element (< _array_index (- (`KismetArrayLibrary.Array_Length` _outpoints) 1))) (`local.TraceChannel`) (`local.TraceComplex`) (`local.ActorsToIgnore`) (`local.DrawDebugType`) (`local.IgnoreSelf`) (`local.TraceColor`) (`local.TraceHitColor`) (`local.DrawTime`)))
    (for _array_element_2 _outhits
      (`KismetArrayLibrary.Array_Add` (`local.AllHits`) _array_element_2)))
  (return (`local.AllHits`)))