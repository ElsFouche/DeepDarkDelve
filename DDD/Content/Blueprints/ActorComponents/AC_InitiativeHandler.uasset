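; Actor component that supplies a unit's turn-order initiative, along with default answers for related queries.
; GetInitiative reads the owner's AC_UnitStatsManager, subtracts a resource from one stat, divides by a second stat, then converts to double.
; It returns -1 when the manager is missing or the divisor is zero.
; Exhaustion, startup exclusion, AI control, faction, icon, name and puppet queries return fixed or empty placeholders.
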(fn `CheckIfExhausted`
  (returns (bExhausted :type Boolean))
  (return false))

(fn `DoNotAddToStartupInitiative`
  (returns (bDoNotAdd :type Boolean))
  (return false))

(fn `GetAiControlled`
  (returns (bAiControlled :type Boolean))
  (return false))

(fn `GetFaction`
  (returns (Faction :type "/Game/AdvancedTurnBasedTileToolkit/Core/Units/EFaction Enum"))
  (return "NewEnumerator3"))

(fn `GetInitiative`
  (returns (Initiative :type "Float (double-precision)"))
  (bind _returnvalue (`Actor.GetComponentByClass` (`self.GetOwner`) "/Game/Blueprints/ActorComponents/AC_UnitStatsManager.AC_UnitStatsManager_C"))
  (bind _value (`/Game/Blueprints/ActorComponents/AC_UnitStatsManager.GetStat` _returnvalue "NewEnumerator9"))
  (`/Engine/EditorBlueprintResources/StandardMacros.IsValid` _returnvalue
    (:`Is Valid`
      (if (!= _value 0)
        (return (`KismetMathLibrary.Conv_IntToDouble` (/ (- (`/Game/Blueprints/ActorComponents/AC_UnitStatsManager.GetStat` _returnvalue "NewEnumerator10") (`/Game/Blueprints/ActorComponents/AC_UnitStatsManager.GetResource` _returnvalue "NewEnumerator2")) _value)))
        (else
          _)))
    (:`Is Not Valid`
      _))
  (return -1.0))

(fn `GetInitiativeIcon`
  (returns (Icon :type "Texture2D Object Reference"))
  (return null))

(fn `GetInitiativeName`
  (returns (Name :type Name))
  (return "None"))

(fn `GetPuppet`
  (returns (Puppet :type "Actor Object Reference"))
  (return null))