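; Actor component that manages a unit's stats and its HP, FP and AP resources.
; Modifiers are stored per source; adding one, or cleaning up those with invalid sources, can flag the cached stats as outdated.
; UpdateCurrentStats lazily rebuilds the cache from base values plus all modifiers, on BeginPlay and before resource changes.
; Resource adjustments are clamped between zero and their maximum stat, while GetStat reads the cache without refreshing it.
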(event `self.ReceiveBeginPlay`
  (`self.UpdateCurrentStats`))

(event `AddStatModifier`
  (params (Source :type "Object Object Reference") (StatFragment :type "/Game/Blueprints/Fragments/BP_StatFragment Object Reference"))
  ; Adds a stat modifier from a particular source
  (`BlueprintMapLibrary.Map_Add` (`self.StatModifiers`) Source StatFragment)
  (set `self.IsStatsUpdated` false))

(event `StatModifierCleanup`
  (bind _statmodifiers (`self.StatModifiers`))
  ; Removes any stat modifiers whose sources are no longer valid
  (bind _keys (`BlueprintMapLibrary.Map_Keys` _statmodifiers))
  (bind _arrayelement (`/Game/Blueprints/Libraries/BPML_Utilities.ForEachLoop_Real` _keys :!label _label)
    (:`LoopBody`
      (`/Engine/EditorBlueprintResources/StandardMacros.IsValid` _arrayelement
        (:`Is Valid`
          (goto _label :!via `Continue`))
        (:`Is Not Valid`
          (bind _returnvalue (`BlueprintMapLibrary.Map_Remove` _statmodifiers _arrayelement))
          (set `self.IsStatsUpdated` (not _returnvalue))
          (goto _label :!via `Continue`))))))

(fn `GetResource`
  (params (Stat :type "/Game/Data/Unit/E_UnitResource Enum" :default "NewEnumerator0"))
  (returns (Value :type Integer))
  (return (`BlueprintMapLibrary.Map_Find` (`self.CurrentResources`) Stat)))

(fn `GetStat`
  (params (Stat :type "/Game/Data/Unit/E_UnitStat Enum" :default "NewEnumerator0"))
  (returns (Value :type Integer))
  (return (`BlueprintMapLibrary.Map_Find` (`self.CurrentStats`) Stat)))

(fn `UpdateCurrentResource`
  (params (Resource :type "/Game/Data/Unit/E_UnitResource Enum" :default "NewEnumerator0") (Adjustment :type Integer))
  (locals (MaxResource :type Integer))
  (`self.UpdateCurrentStats`)
  (switch `/Game/Data/Unit/E_UnitResource` Resource
    (:`NewEnumerator0`
      (set `local.MaxResource` (`self.GetStat` "NewEnumerator1")))
    (:`NewEnumerator1`
      (set `local.MaxResource` (`self.GetStat` "NewEnumerator4")))
    (:`NewEnumerator2`
      (set `local.MaxResource` (`self.GetStat` "NewEnumerator7"))))
  (`BlueprintMapLibrary.Map_Add` (`self.CurrentResources`) Resource (`KismetMathLibrary.Clamp` (+ Adjustment (`BlueprintMapLibrary.Map_Find` (`self.CurrentResources`) Resource)) 0 (`local.MaxResource`)))
  (return))

(fn `UpdateCurrentStats`
  (locals (Acc :type Integer))
  (if (`self.IsStatsUpdated`)
    (return)
    (else
      (bind _enumvalue (foreach `/Game/Data/Unit/E_UnitStat` false)
        (:`LoopBody`
          (bind (_value _returnvalue) (`BlueprintMapLibrary.Map_Find` (`self.BaseStats`) _enumvalue))
          (if _returnvalue
            (set `local.Acc` _value)
            (else
              (set `local.Acc` 0)))
          (bind _values (`BlueprintMapLibrary.Map_Values` (`self.StatModifiers`)))
          (for _array_element _values
            (bind (_value_2 _returnvalue_2) (`BlueprintMapLibrary.Map_Find` (`/Game/Blueprints/Fragments/BP_StatFragment.StatModifiers` _array_element) _enumvalue))
            (if _returnvalue_2
              (set `local.Acc` (+ _value_2 (`local.Acc`)))))
          (`BlueprintMapLibrary.Map_Add` (`self.CurrentStats`) _enumvalue (`local.Acc`)))
        (:`then`
          (set `self.IsStatsUpdated` true)
          (return))))))