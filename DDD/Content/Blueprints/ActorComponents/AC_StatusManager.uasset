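; Actor component that manages status effects on its owning actor in turn-based combat.
; AddStatus rejects immune classes, initializes the status, then merges it into an existing one of that class or appends it.
; Statuses can be looked up or removed by class, and Cleanup removes those without stacks.
; Combat clock, turn begin and turn end events are forwarded to every status; a debug event prints test status strings.
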(event `PrintTestStringIfFound`
  (bind _thecount (`self.TheCount`))
  ;[9.585 0.1635 -1.128 9.557 24] DEBUG: for testing adding, removing, and merging using TestStatus1
  (bind _arrayelement (`/Game/Blueprints/Libraries/BPML_Utilities.ForEachLoop_Real` (`self.Status`) :!label _label)
    (:`LoopBody`
      (bind _asbp_test_status_1 (cast `/Game/Blueprints/StatusEffects/BP_TestStatus1` _arrayelement)
        (:`then`
          (`KismetSystemLibrary.PrintString` (`KismetStringLibrary.Concat_StrStr` (`KismetStringLibrary.Conv_IntToString` _thecount) ". " (`/Game/Blueprints/StatusEffects/BP_TestStatus1.teststring` _asbp_test_status_1)) true true (struct :`G` 0.66 :`B` 1.0 :`A` 1.0) 60.0))
        (:`CastFailed`
          (goto _label :!via `Continue`))))
    (:`Completed`
      (`KismetSystemLibrary.PrintString` (`KismetStringLibrary.Concat_StrStr` (`KismetStringLibrary.Conv_IntToString` (`self.TheCount`)) ". " "teststatus1 not found in current status array") true true (struct :`G` 0.66 :`B` 1.0 :`A` 1.0) 60.0)))
  (`/Engine/EditorBlueprintResources/StandardMacros.IncrementInt` _thecount))

(event `AddStatus`
  (params (StatusToAdd :type "/Game/Blueprints/StatusEffects/BP_ParentStatus Object Reference"))
  (bind _returnvalue (`GameplayStatics.GetObjectClass` StatusToAdd))
  (if (not (`KismetArrayLibrary.Array_Contains` (`self.StatusImmunities`) _returnvalue))
    (`/Game/Blueprints/StatusEffects/BP_ParentStatus.Initialize` StatusToAdd null)
    (set `/Game/Blueprints/StatusEffects/BP_ParentStatus.Manager` self StatusToAdd)
    (bind (_arrayelement _arrayindex) (`/Game/Blueprints/Libraries/BPML_Utilities.ForEachLoop_Real` (`self.Status`) :!label _label_2)
      (:`LoopBody`
        (if (`GameplayStatics.ObjectIsA` _arrayelement _returnvalue)
          (bind _newstatus (`/Game/Blueprints/StatusEffects/BP_ParentStatus.MergeStatus` _arrayelement StatusToAdd))
          (`KismetArrayLibrary.Array_Set` (`self.Status`) _arrayindex _newstatus)
          (else
            (goto _label_2 :!via `Continue`))))
      (:`Completed`
        (`KismetArrayLibrary.Array_Add` (`self.Status`) StatusToAdd)))))

(event `self.ReceiveBeginPlay`
  (set `self.ParentReference` (`self.GetOwner`)))

(event `RemoveStatus`
  (params (StatusToEnd :type "/Game/Blueprints/StatusEffects/BP_ParentStatus Class Reference"))
  (bind (_arrayelement _arrayindex) (`/Game/Blueprints/Libraries/BPML_Utilities.ForEachLoop_Real` (`self.Status`) :!label _label_3)
    (:`LoopBody`
      (if (`GameplayStatics.ObjectIsA` _arrayelement StatusToEnd)
        (`KismetArrayLibrary.Array_Remove` (`self.Status`) _arrayindex)
        (else
          (goto _label_3 :!via `Continue`))))))

(event `Cleanup`
  (bind (_arrayelement _arrayindex) (`/Game/Blueprints/Libraries/BPML_Utilities.ForEachLoop_Real` (`self.Status`) :!label _label_4)
    (:`LoopBody`
      (if (<= (`/Game/Blueprints/StatusEffects/BP_ParentStatus.Stacks` _arrayelement) 0)
        (`KismetArrayLibrary.Array_Remove` (`self.Status`) _arrayindex)
        (goto _label_4 :!via `Continue`)
        (else
          (goto _label_4 :!via `Continue`))))))

(event `RunOnCombatClockUpdate`
  (params (Ticks :type Integer))
  (for _array_element (`self.Status`)
    (`/Game/Blueprints/StatusEffects/BP_ParentStatus.OnClockUpdate` _array_element Ticks)))

(event `RunOnParentBeginTurn`
  (for _array_element (`self.Status`)
    (`/Game/Blueprints/StatusEffects/BP_ParentStatus.OnTurnBegin` _array_element)))

(event `RunOnParentEndTurn`
  (for _array_element (`self.Status`)
    (`/Game/Blueprints/StatusEffects/BP_ParentStatus.OnTurnEnd` _array_element)))

(fn `GetStatus`
  (params (StatusType :type "/Game/Blueprints/StatusEffects/BP_ParentStatus Class Reference"))
  (returns (___ :type "/Game/Blueprints/StatusEffects/BP_ParentStatus Object Reference") (success :type Boolean))
  (bind (_arrayelement _arrayindex) (`/Game/Blueprints/Libraries/BPML_Utilities.ForEachLoop_Real` (`self.Status`) :!label _label)
    (:`LoopBody`
      (if (`GameplayStatics.ObjectIsA` _arrayelement StatusType)
        (return (`|GetArrayItem` (`self.Status`) _arrayindex) true)
        (else
          (goto _label :!via `Continue`))))
    (:`Completed`
      (return null false))))