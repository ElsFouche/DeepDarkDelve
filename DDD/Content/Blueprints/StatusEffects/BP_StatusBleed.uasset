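; Bleed status effect that damages its owning unit at the start of each turn and wears off over time.
; Each tick lowers a resource through the unit's stats manager, combining a percentage of a stat with a stack-scaled percentage of the current resource, rounded down.
; Stacks drop each turn, and the status removes itself through its manager once they fall below zero.
; Merging another bleed adds its stacks to this one.
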(event `self.OnTurnBegin`
  (bind _returnvalue (`Actor.GetComponentByClass` (`ActorComponent.GetOwner` (`self.Manager`)) "/Game/Blueprints/ActorComponents/AC_UnitStatsManager.AC_UnitStatsManager_C"))
  ; get the owner's stats, and hurt them
  (`/Game/Blueprints/ActorComponents/AC_UnitStatsManager.UpdateCurrentResource` _returnvalue "NewEnumerator0" (`KismetMathLibrary.FFloor` (+ (* (`/Game/Blueprints/ActorComponents/AC_UnitStatsManager.GetStat` _returnvalue "NewEnumerator1") -0.01) (* (`/Game/Blueprints/ActorComponents/AC_UnitStatsManager.GetResource` _returnvalue "NewEnumerator0") (* (`self.Stacks`) -0.025)))))
  (bind _result (`/Engine/EditorBlueprintResources/StandardMacros.DecrementInt` (`self.Stacks`))
    (:`  `
      (if (< _result 0)
        (`/Game/Blueprints/ActorComponents/AC_StatusManager.RemoveStatus` (`self.Manager`) (`GameplayStatics.GetObjectClass` self))))))

(fn `MergeStatus`
  (params (`Other Status` :type "/Game/Blueprints/StatusEffects/BP_ParentStatus Object Reference"))
  (returns (NewStatus :type "/Game/Blueprints/StatusEffects/BP_ParentStatus Object Reference"))
  (bind _asbp_status_bleed (cast `/Game/Blueprints/StatusEffects/BP_StatusBleed` `Other Status`)
    (:`then`
      (set `self.Stacks` (+ (`/Game/Blueprints/StatusEffects/BP_ParentStatus.Stacks` _asbp_status_bleed) (`self.Stacks`))))
    (:`CastFailed`
      _))
  (return self))