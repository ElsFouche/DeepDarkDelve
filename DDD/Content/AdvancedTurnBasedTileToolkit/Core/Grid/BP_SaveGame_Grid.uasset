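; BP_SaveGame_Grid is a save-game container for the grid data of the turn-based tile toolkit.
; StoreGridVariables copies the grid locations, edges and height map levels from a grid manager into its own variables.
; LoadStoredVariablesOntoGrid writes the same three variables back onto a given grid, with no processing in either direction.
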(fn `LoadStoredVariablesOntoGrid`
  (params (Grid :type "/Game/AdvancedTurnBasedTileToolkit/Core/Grid/BP_GridManager Object Reference"))
  (set `/Game/AdvancedTurnBasedTileToolkit/Core/Grid/BP_GridManager.GridLocations` (`self.GridLocations`) Grid)
  (set `/Game/AdvancedTurnBasedTileToolkit/Core/Grid/BP_GridManager.GridEdges` (`self.GridEdges`) Grid)
  (set `/Game/AdvancedTurnBasedTileToolkit/Core/Grid/BP_GridManager.HeightMapLevels` (`self.HeightMapLevels`) Grid)
  (return))

(fn `StoreGridVariables`
  (params (GridManager :type "/Game/AdvancedTurnBasedTileToolkit/Core/Grid/BP_GridManager Object Reference"))
  (set `self.GridLocations` (`/Game/AdvancedTurnBasedTileToolkit/Core/Grid/BP_GridManager.GridLocations` GridManager))
  (set `self.GridEdges` (`/Game/AdvancedTurnBasedTileToolkit/Core/Grid/BP_GridManager.GridEdges` GridManager))
  (set `self.HeightMapLevels` (`/Game/AdvancedTurnBasedTileToolkit/Core/Grid/BP_GridManager.HeightMapLevels` GridManager))
  (return))